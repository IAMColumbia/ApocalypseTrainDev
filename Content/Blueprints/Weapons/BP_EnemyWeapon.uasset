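; Enemy weapon actor that damages the player character on contact.
; On actor overlap it checks for the Player tag, casts to BP_MyCharacter and calls TakeDamage with its Damage value when CanDamage is set.
; A tracked Player array with a DamagePlayers loop and a debug sphere draw are left disconnected; only the sphere's end-overlap still removes entries from the array, and Tick does nothing.
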(event OnComponentEndOverlap(Sphere)
  (params (OverlappedComponent :type Primitive%20Component%20Object%20Reference) (OtherActor :type Actor%20Object%20Reference) (OtherComp :type Primitive%20Component%20Object%20Reference) (OtherBodyIndex :type Integer))
  (if (Actor|ActorHasTag OtherActor "Player")
    (bind _asbp_my_character (Utilities|Casting|CastToBP_MyCharacter OtherActor))
    (Utilities|Array|RemoveItem (Variables|Default|GetPlayer) _asbp_my_character)))

(event EventBeginPlay)

(event Collision|EventActorBeginOverlap
  (params (OtherActor :type Actor%20Object%20Reference))
  (Utilities|IsValid OtherActor
    (:Is%20Valid
      (if (Actor|ActorHasTag OtherActor "Player")
        (bind _asbp_my_character (Utilities|Casting|CastToBP_MyCharacter OtherActor))
        (if (Variables|Default|GetcanDamage)
          (Class|MyCharacter|TakeDamage _asbp_my_character (Variables|Default|GetDamage)))))))

(event EventTick
  (params (DeltaSeconds :type Float%20%28single-precision%29))
  (Utilities|FlowControl|Sequence))

(fn ConstructionScript)

(fn DamagePlayers
  (for _array_element (Variables|Default|GetPlayer)
    (if (Variables|Default|GetcanDamage)
      (Class|MyCharacter|TakeDamage _array_element (Variables|Default|GetDamage)))))