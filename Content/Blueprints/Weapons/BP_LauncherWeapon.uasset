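; Launcher weapon Blueprint that adds cosmetic feedback whenever a shot is fired.
; NotifyFiredShot plays force feedback on the owning player's controller and a randomly pitch-shifted launch sound attached to BulletSpawn.
; It fakes recoil by setting the actor's relative Y location, then setting it to the opposite offset after a short delay.
; A muzzle explosion emitter is present but disconnected, so it never spawns.
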(event EventBeginPlay)

(event Collision|EventActorBeginOverlap
  (params (OtherActor :type Actor%20Object%20Reference)))

(event EventTick
  (params (DeltaSeconds :type Float%20%28single-precision%29)))

(event EventNotifyFiredShot
  (Game|Feedback|ClientPlayForceFeedback (Game|GetPlayerController (Class|Weapon|OwnerPlayerIndex)) "/Game/FX/FF_Shoot.FF_Shoot" "None" false false false)
  (Audio|SpawnSoundAttached "/Game/Audio/MetaSounds/Weapons/Launcher_Source.Launcher_Source" (Variables|Default|GetBulletSpawn) "None" "0, 0, 0" "0, 0, 0" "KeepRelativeOffset" false 1.0 (+ (Math|Random|RandomFloatinRange -0.1 0.1) 1.0) 0.0 "/Game/Audio/BasicAttenuation.BasicAttenuation" 0)
  (Transformation|SetActorRelativeLocation (Math|Vector|MakeVector 0.0 2e+01 0.0))
  (Utilities|FlowControl|Delay 0.13)
  (Transformation|SetActorRelativeLocation "0.000000,-20.000000,0.000000"))

(fn ConstructionScript)