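; Assault rifle weapon Blueprint that handles the gun's visual, audio and haptic feedback.
; Firing plays controller rumble, a muzzle burst and a brief positional kick, and triggers a persistent attached sound spawned at BeginPlay.
; Stopping sends that sound an end trigger, and owner death calls Play on it.
; Bullet impacts spawn pooled Niagara effects chosen by hit type, while Tick keeps the laser beam's endpoint updated.
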(event EventSpawnBulletVFX
  (params (location :type Vector :default "0, 0, 0") (normal :type Vector :default "0, 0, 0") (type :type Integer))
  (Utilities|FlowControl|Sequence
    (:then_0
      (switch int type
        (:Default
          (Variables|Default|SetSystem%20To%20Spawn "/Game/VFX/NS_GunHit.NS_GunHit" :!label _label))
        (:0
          (goto _label))
        (:1
          (Variables|Default|SetSystem%20To%20Spawn "/Game/VFX/NS_GunHitBrown.NS_GunHitBrown"))))
    (:then_1
      (Niagara|SpawnSystematLocation (Variables|Default|GetSystem%20To%20Spawn) location (Math|Conversions|RotationFromXVector normal) "1.000000,1.000000,1.000000" true true "AutoRelease"))))

(event Collision|EventActorBeginOverlap
  (params (OtherActor :type Actor%20Object%20Reference)))

(event EventNotifyStoppedShooting
  (Class|AudioParameterControllerInterface|SetTriggerParameter (Variables|Default|GetShotAudioSource) "End"))

(event EventTick
  (params (DeltaSeconds :type Float%20%28single-precision%29))
  (CallFunction|UpdateLaserBeam))

(event EventNotifyFiredShot
  (Game|Feedback|ClientPlayForceFeedback (Game|GetPlayerController (Class|Weapon|OwnerPlayerIndex)) "/Game/FX/FF_Shoot.FF_Shoot" "None" false false false)
  (Effects|SpawnEmitterAttached "/Game/StarterContent/Particles/P_ExplosionMuzzle.P_ExplosionMuzzle" (Variables|Default|GetBulletSpawn) "None" "0, 0, 0" "0, 0, 0" "0.300000,0.300000,0.300000" "SnapToTarget")
  (Class|AudioParameterControllerInterface|SetTriggerParameter (Variables|Default|GetShotAudioSource) "TriggerShot")
  (Transformation|SetActorRelativeLocation (Math|Vector|MakeVector 0.0 -7.0 0.0))
  (Utilities|FlowControl|Delay 0.1)
  (Transformation|SetActorRelativeLocation "0.000000,7.000000,0.000000"))

(event EventBeginPlay
  (bind _returnvalue (Audio|SpawnSoundAttached "/Game/Audio/MetaSounds/AR_Source.AR_Source" (Variables|Default|GetBulletSpawn) "None" "0, 0, 0" "0, 0, 0" "KeepRelativeOffset" false 1.0 1.0 0.0 "/Game/Audio/BasicAttenuation.BasicAttenuation" 0))
  (Variables|Default|SetShotAudioSource _returnvalue))

(event EventOwnerDied
  (Audio|Components|Audio|Play (Variables|Default|GetShotAudioSource) 0.0))

(fn ConstructionScript)

(fn UpdateLaserBeam
  (Effects|Components|ParticleSystem|SetVectorParameter (Variables|Default|GetLaserBeam) "Beam End" (Class|Weapon|GetBeamEnd)))