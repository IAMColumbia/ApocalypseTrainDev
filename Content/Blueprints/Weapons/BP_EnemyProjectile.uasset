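; BP_EnemyProjectile is a physics-driven grenade projectile that explodes on impact, damaging player characters and shatterable obstacles.
; Launch sets the grenade's velocity while a timeline animates its scale relative to the initial size.
; Explosion plays pitch-varied sound and a particle effect, damages actors overlapping its radius, then destroys itself.
; A visibility trace shields obstacles behind cover; characters take damage regardless, as their cover check and the cook-time fuse are disconnected.
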(event OnComponentHit(Grenade)
  (params (HitComponent :type Primitive%20Component%20Object%20Reference) (OtherActor :type Actor%20Object%20Reference) (OtherComp :type Primitive%20Component%20Object%20Reference) (NormalImpulse :type Vector :default "0, 0, 0") (Hit :type Hit%20Result%20Structure%20%28by%20ref%29))
  (CallFunction|Explosion))

(event EventBeginPlay
  (Variables|Default|SetinitalSize (Transformation|GetWorldScale (Variables|Default|GetGrenade))))

(event Collision|EventActorBeginOverlap
  (params (OtherActor :type Actor%20Object%20Reference)))

(event EventTick
  (params (DeltaSeconds :type Float%20%28single-precision%29)))

(event EventLaunch
  (params (Direction :type Vector :default "0, 0, 0"))
  (bind _grenade (Variables|Default|GetGrenade))
  (Utilities|FlowControl|Sequence
    (:then_0
      (bind _scale (Timeline|ScaleGrenade PlayFromStart)
        (:Update
          (Transformation|SetWorldScale3D _grenade (* (Variables|Default|GetinitalSize) _scale)))
        (:Finished
          (Transformation|SetWorldScale3D _grenade (Variables|Default|GetinitalSize)))))
    (:then_1
      (Physics|SetPhysicsLinearVelocity (Variables|Default|GetGrenade) Direction false "None"))))

(fn ConstructionScript)

(fn Explosion
  (bind _explosionradus (Variables|Default|GetExplosionRadus))
  (Audio|SpawnSoundatLocation "/Game/Audio/MetaSounds/Grenade_Source.Grenade_Source" (Transformation|GetWorldLocation (Variables|Default|GetGrenade)) "0, 0, 0" 1.0 (+ (Math|Random|RandomFloatinRange -0.1 0.1) 1.0) 0.0 "/Game/Audio/BasicAttenuation.BasicAttenuation" 0)
  (Utilities|FlowControl|Sequence
    (:then_0
      (Effects|SpawnEmitteratLocation "/Game/StarterContent/Particles/P_Explosion.P_Explosion" (+ (Transformation|GetWorldLocation (Variables|Default|GetGrenade)) "0.000000,0.000000,80.000000")))
    (:then_1
      (for _array_element (Collision|GetOverlappingActors _explosionradus "/Script/Prototype0Unreal.MyCharacter" :!class /Script/Engine.PrimitiveComponent)
        (bind _asmy_character (Utilities|Casting|CastToMyCharacter _array_element))
        (Class|MyCharacter|TakeDamage _asmy_character (Variables|Default|GetDamage))))
    (:then_2
      (for _array_element_2 (Collision|GetOverlappingActors _explosionradus "/Game/Blueprints/BP_Shatter.BP_Shatter_C" :!class /Script/Engine.PrimitiveComponent)
        (bind _asbp_shatter (Utilities|Casting|CastToBP_Shatter _array_element_2))
        (bind _hascover (CallFunction|HasCover _asbp_shatter))
        (if (not _hascover)
          (Class|Obstacle|DamageObstacle _asbp_shatter (* (Variables|Default|GetDamage) (Variables|Default|GetObstacleDamageMult))))))
    (:then_3
      (Actor|DestroyActor))))

(fn HasCover
  (params (Actor :type Actor%20Object%20Reference))
  (bind _returnvalue (Transformation|GetActorLocation Actor))
  (bind _grenade (Variables|Default|GetGrenade))
  (bind _actors_to_ignore (Variables|Default|GetActors%20to%20Ignore))
  (bind _returnvalue_2 (Transformation|GetWorldLocation _grenade))
  (Utilities|IsValid Actor
    (:Is%20Valid
      (Utilities|Array|Add _actors_to_ignore Actor)
      (Utilities|Array|Add _actors_to_ignore self)
      (bind _returnvalue_3 (Collision|LineTraceByChannel _returnvalue _returnvalue_2 "TraceTypeQuery1" false (Variables|Default|GetActors%20to%20Ignore) "None"))
      (return _returnvalue_3 (Math|Vector|Normalize (- _returnvalue_2 _returnvalue))))))