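; AR weapon projectile Blueprint that despawns itself when its Box collision overlaps another actor.
; ShouldDespawn ignores actors carrying any tag in TagsToIgnore; any other overlap calls Despawn, defined outside these graphs, after a brief delay.
; The graphs apply no damage or movement: BeginPlay and Tick are empty, and a leftover SetActorLocation node is never executed.
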(event OnComponentBeginOverlap(Box)
  (params (OverlappedComponent :type Primitive%20Component%20Object%20Reference) (OtherActor :type Actor%20Object%20Reference) (OtherComp :type Primitive%20Component%20Object%20Reference) (OtherBodyIndex :type Integer) (bFromSweep :type Boolean) (SweepResult :type Hit%20Result%20Structure%20%28by%20ref%29))
  (bind _shoulddespawn (CallFunction|ShouldDespawn OtherActor))
  (if _shoulddespawn
    (Utilities|FlowControl|Delay 0.05)
    (Class|Projectile|Despawn)))

(event EventBeginPlay)

(event Collision|EventActorBeginOverlap
  (params (OtherActor :type Actor%20Object%20Reference)))

(event EventTick
  (params (DeltaSeconds :type Float%20%28single-precision%29)))

(fn ConstructionScript)

(fn ShouldDespawn
  (params (Actor :type Actor%20Object%20Reference))
  (for _array_element (Variables|Default|GetTagsToIgnore)
    (if (Actor|ActorHasTag Actor (Utilities|String|StringToName _array_element))
      (return false)))
  (return true))