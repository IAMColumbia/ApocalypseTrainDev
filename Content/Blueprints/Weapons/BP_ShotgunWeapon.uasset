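; Shotgun weapon Blueprint that supplies firing feedback and a laser beam.
; Each tick, UpdateLaser sets the LaserBeam "Beam End" vector parameter from GetBeamEnd.
; NotifyFiredShot plays force feedback on the owning player's controller and attaches a muzzle effect and a pitch-randomized shot sound to BulletSpawn.
; The graphs shown hold no projectile or damage logic.
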(event EventBeginPlay)

(event Collision|EventActorBeginOverlap
  (params (OtherActor :type Actor%20Object%20Reference)))

(event EventTick
  (params (DeltaSeconds :type Float%20%28single-precision%29))
  (CallFunction|UpdateLaser))

(event EventNotifyFiredShot
  (Game|Feedback|ClientPlayForceFeedback (Game|GetPlayerController (Class|Weapon|OwnerPlayerIndex)) "/Game/FX/FF_Shoot.FF_Shoot" "None" false false false)
  (Effects|SpawnEmitterAttached "/Game/StarterContent/Particles/P_ExplosionMuzzle.P_ExplosionMuzzle" (Variables|Default|GetBulletSpawn) "None" "0, 0, 0" "0, 0, 0" "0.300000,0.300000,0.300000" "SnapToTarget")
  (Audio|SpawnSoundAttached "/Game/Audio/MetaSounds/Shotgun_Source.Shotgun_Source" (Variables|Default|GetBulletSpawn) "None" "0, 0, 0" "0, 0, 0" "KeepRelativeOffset" false 1.2 (+ (Math|Random|RandomFloatinRange -0.1 0.1) 1.0) 0.0 "/Game/Audio/BasicAttenuation.BasicAttenuation" 0))

(fn ConstructionScript)

(fn UpdateLaser
  (Effects|Components|ParticleSystem|SetVectorParameter (Variables|Default|GetLaserBeam) "Beam End" (Class|Weapon|GetBeamEnd)))