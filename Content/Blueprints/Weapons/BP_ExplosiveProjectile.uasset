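; Physics grenade projectile that, once launched, plays a scale animation and explodes on hit or after a cook time.
; The explosion plays controller rumble, sound, particles and a fading decal, then destroys the actor.
; It damages and knocks back overlapping AI_Enemy actors, calling KilledEnemy on kills, and deals multiplied damage to BP_Shatter obstacles.
; A HasCover visibility line trace gates both kinds of damage.
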(event OnComponentHit(Grenade)
  (params (HitComponent :type Primitive%20Component%20Object%20Reference) (OtherActor :type Actor%20Object%20Reference) (OtherComp :type Primitive%20Component%20Object%20Reference) (NormalImpulse :type Vector :default "0, 0, 0") (Hit :type Hit%20Result%20Structure%20%28by%20ref%29))
  (CallFunction|Explosion))

(event EventBeginPlay
  (Variables|Default|SetinitalSize (Transformation|GetWorldScale (Variables|Default|GetGrenade))))

(event Collision|EventActorBeginOverlap
  (params (OtherActor :type Actor%20Object%20Reference)))

(event EventTick
  (params (DeltaSeconds :type Float%20%28single-precision%29)))

(event EventLaunch
  (params (Direction :type Vector :default "0, 0, 0"))
  (bind _grenade (Variables|Default|GetGrenade))
  (Utilities|FlowControl|Sequence
    (:then_0
      (bind _scale (Timeline|ScaleGrenade PlayFromStart)
        (:Update
          (Transformation|SetWorldScale3D _grenade (* (Variables|Default|GetinitalSize) _scale)))
        (:Finished
          (Transformation|SetWorldScale3D _grenade (Variables|Default|GetinitalSize)))))
    (:then_1
      (Physics|SetPhysicsLinearVelocity (Variables|Default|GetGrenade) (* Direction (Variables|Default|GetVelocity)) false "None")
      (Utilities|FlowControl|Delay (Variables|Default|GetCookTime))
      (CallFunction|Explosion))))

(fn ConstructionScript)

(fn Explosion
  (bind _explosionradus (Variables|Default|GetExplosionRadus))
  (Game|Feedback|ClientPlayForceFeedback (Game|GetPlayerController (Variables|Default|GetFiredPlayerIndex)) "/Game/FX/FF_Shoot.FF_Shoot" "None" false false false)
  (Audio|SpawnSoundatLocation "/Game/Audio/MetaSounds/Grenade_Source.Grenade_Source" (Transformation|GetWorldLocation (Variables|Default|GetGrenade)) "0, 0, 0" 1.0 (+ (Math|Random|RandomFloatinRange -0.1 0.1) 1.0) 0.0 "/Game/Audio/BasicAttenuation.BasicAttenuation" 0)
  (CallFunction|SpawnDecal)
  (Utilities|FlowControl|Sequence
    (:then_0
      (Effects|SpawnEmitteratLocation "/Game/StarterContent/Particles/P_Explosion.P_Explosion" (+ (Transformation|GetWorldLocation (Variables|Default|GetGrenade)) "0.000000,0.000000,80.000000")))
    (:then_1
      (for _array_element (Collision|GetOverlappingActors _explosionradus "/Game/Blueprints/Enemies/AI_Enemy.AI_Enemy_C" :!class /Script/Engine.PrimitiveComponent)
        (bind _asai_enemy (Utilities|Casting|CastToAI_Enemy _array_element))
        (bind (_hascover _directionfromgrenade) (CallFunction|HasCover _asai_enemy))
        (if (not _hascover)
          (bind _returnvalue (Class|EnemyCharacter|TakeDamage _asai_enemy 0.0 (Variables|Default|GetDamage) "0, 0, 0" 0.0 true))
          (Default|Knockback _asai_enemy _directionfromgrenade (Variables|Default|GetKnock%20Force))
          (if _returnvalue
            (Class|ExplosiveProjectile|KilledEnemy)))))
    (:then_2
      (for _array_element_2 (Collision|GetOverlappingActors _explosionradus "/Game/Blueprints/BP_Shatter.BP_Shatter_C" :!class /Script/Engine.PrimitiveComponent)
        (bind _asbp_shatter (Utilities|Casting|CastToBP_Shatter _array_element_2))
        (bind _hascover_2 (CallFunction|HasCover _asbp_shatter))
        (if (not _hascover_2)
          (Class|Obstacle|DamageObstacle _asbp_shatter (* (Variables|Default|GetDamage) (Variables|Default|GetObstacleDamageMult))))))
    (:then_3
      (Actor|DestroyActor))))

(fn HasCover
  (params (Actor :type Actor%20Object%20Reference))
  (bind _returnvalue (Transformation|GetActorLocation))
  (bind _grenade (Variables|Default|GetGrenade))
  (bind _returnvalue_2 (Transformation|GetWorldLocation _grenade))
  (Utilities|IsValid Actor
    (:Is%20Valid
      (Utilities|Array|Add (Variables|Default|GetActors%20to%20Ignore) Actor)
      (bind _returnvalue_3 (Collision|LineTraceByChannel _returnvalue _returnvalue_2 "TraceTypeQuery1" false (Variables|Default|GetActors%20to%20Ignore) "None"))
      (return _returnvalue_3 (Math|Vector|Normalize (- _returnvalue_2 _returnvalue))))))

(fn SpawnDecal
  (bind _returnvalue (Rendering|Decal|SpawnDecalatLocation "/Game/Decals/ExplosionHole_Mat.ExplosionHole_Mat" (Math|Conversions|ToVector(Float) (Math|Float|MakeLiteralFloat 8e+01)) (Transformation|GetWorldLocation (Variables|Default|GetGrenade)) (Math|Rotator|MakeRotator 0.0 -9e+01 (Math|Random|RandomFloatinRange -1.8e+02 1.8e+02)) 0.0))
  (Rendering|Components|Decal|SetFadeOut _returnvalue 2.0 3.0 true))