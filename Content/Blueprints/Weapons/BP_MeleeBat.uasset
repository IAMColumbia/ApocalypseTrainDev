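; Melee bat weapon Blueprint that handles hitbox toggling and sound for swings and hits.
; It caches the Box's collision mode on BeginPlay, restores it on Attacking along with an attached swing sound, and disables it on Idle.
; HitEnemy plays an impact sound at the bat mesh, while HitObstacle is empty and its stone-hit sound and delay nodes are left disconnected.
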(event EventBeginPlay
  (Variables|Default|SetDefCollision (Collision|GetCollisionEnabled (Variables|Default|GetBox))))

(event Collision|EventActorBeginOverlap
  (params (OtherActor :type Actor%20Object%20Reference)))

(event EventTick
  (params (DeltaSeconds :type Float%20%28single-precision%29)))

(event EventAttacking
  (bind _bat_gameready (Variables|Default|GetBat_GameReady))
  (Collision|SetCollisionEnabled (Variables|Default|GetBox) (Variables|Default|GetDefCollision))
  (Audio|SpawnSoundAttached "/Game/Audio/MetaSounds/Weapons/MeleeBat_Source.MeleeBat_Source" _bat_gameready "None" (Transformation|GetWorldLocation _bat_gameready) "0, 0, 0" "SnapToTarget" false 1.0 1.0 0.0 "/Game/Audio/BasicAttenuation.BasicAttenuation" 0))

(event EventIdle
  (Collision|SetCollisionEnabled (Variables|Default|GetBox) "NoCollision"))

(event EventHitObstacle)

(event EventHitEnemy
  (Audio|PlaySoundatLocation "/Game/Audio/MetaSounds/Weapons/MS_Bat_HitEnemy.MS_Bat_HitEnemy" (Transformation|GetWorldLocation (Variables|Default|GetBat_GameReady)) "0, 0, 0" 1.0 1.0 0.0 0 0 0 0))

(fn ConstructionScript)