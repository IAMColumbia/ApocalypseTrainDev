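; Sniper weapon Blueprint that supplies shot feedback, impact effects and a laser sight.
; Tick calls UpdateLaser, which feeds GetBeamEnd into the LaserBeam's end parameter.
; NotifyFiredShot plays controller rumble and a pitch-randomized sound, then fakes recoil by shifting the actor's relative location before and after a short delay.
; SpawnBulletVFX picks a default, brown or blood Niagara hit effect by type and spawns it pooled, aligned to the surface normal.
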(event EventSpawnBulletVFX
  (params (location :type Vector :default "0, 0, 0") (normal :type Vector :default "0, 0, 0") (type :type Integer))
  (Utilities|FlowControl|Sequence
    (:then_0
      (switch int type
        (:Default
          (Variables|Components|SetSystem%20To%20Spawn "/Game/VFX/NS_GunHit.NS_GunHit" :!label _label))
        (:0
          (goto _label))
        (:1
          (Variables|Components|SetSystem%20To%20Spawn "/Game/VFX/NS_GunHitBrown.NS_GunHitBrown"))
        (:2
          (Variables|Components|SetSystem%20To%20Spawn "/Game/VFX/NS_GunHitBlood.NS_GunHitBlood"))))
    (:then_1
      (Niagara|SpawnSystematLocation (Variables|Components|GetSystem%20To%20Spawn) location (Math|Conversions|RotationFromXVector normal) "1.000000,1.000000,1.000000" true true "AutoRelease"))))

(event Collision|EventActorBeginOverlap
  (params (OtherActor :type Actor%20Object%20Reference)))

(event EventTick
  (params (DeltaSeconds :type Float%20%28single-precision%29))
  (CallFunction|UpdateLaser))

(event EventBeginPlay)

(event EventNotifyFiredShot
  (Game|Feedback|ClientPlayForceFeedback (Game|GetPlayerController (Class|Weapon|OwnerPlayerIndex)) "/Game/FX/FF_Shoot.FF_Shoot" "None" false false false)
  (Audio|SpawnSoundAttached "/Game/Audio/AudioFiles/Weapons/Sniper1.Sniper1" (Variables|Default|GetBulletSpawn) "None" "0, 0, 0" "0, 0, 0" "KeepRelativeOffset" false 1.0 (+ (Math|Random|RandomFloatinRange -0.1 0.1) 1.0) 0.0 "/Game/Audio/BasicAttenuation.BasicAttenuation" 0)
  (Transformation|SetActorRelativeLocation (Math|Vector|MakeVector 0.0 2e+01 0.0))
  (Utilities|FlowControl|Delay 0.13)
  (Transformation|SetActorRelativeLocation "0.000000,-20.000000,0.000000"))

(fn ConstructionScript)

(fn UpdateLaser
  (Effects|Components|ParticleSystem|SetVectorParameter (Variables|Default|GetLaserBeam) "Beam End" (Class|Weapon|GetBeamEnd)))