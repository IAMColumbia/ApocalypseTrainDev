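; Destructible barricade obstacle with a floating health bar and feedback for hits and destruction.
; On damage, it updates the bar, flashes a dynamic material white, shakes the mesh scale via timeline, and plays a sound.
; A second timeline animates bar opacity, while Tick pins its yaw to a fixed angle during display.
; On destruction, it spawns a poof particle, plays a sound, stops both timelines and destroys itself.
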(event EventBeginPlay
  (CallFunction|UpdateHealthBar)
  (CallFunction|SetFashMat)
  (Variables|Default|SetScale (Transformation|GetWorldScale (Variables|Default|GetBarricade)))
  (bind _aswb_health_bar (Utilities|Casting|CastToWB_HealthBar (UserInterface|GetWidget (Variables|Default|Gethb))))
  (Default|SetOpacity _aswb_health_bar 0.0))

(event Collision|EventActorBeginOverlap
  (params (OtherActor :type Actor%20Object%20Reference)))

(event EventNotifyDamageObstacle
  (params (damage :type Float%20%28single-precision%29))
  (bind _hb (Variables|Default|Gethb))
  (bind _hitsound (Variables|Default|GetHitSound))
  (bind _barricade (Variables|Default|GetBarricade))
  (bind _flashmat (Variables|Default|GetFlashMat))
  (bind _returnvalue (UserInterface|GetWidget _hb))
  (Variables|Default|SethealthBarVisible true)
  (Utilities|FlowControl|Sequence
    (:then_0
      (CallFunction|ShowHealthBar)
      (CallFunction|UpdateHealthBar)
      (Utilities|FlowControl|Sequence
        (:then_0
          (Rendering|Material|SetVectorParameterValue _flashmat "FlashVector" (Math|Conversions|ToLinearColor(Vector) (Math|Vector|MakeVector 1.0 1.0 1.0)) :!class /Script/Engine.MaterialInstanceDynamic)
          (Utilities|FlowControl|Delay 0.1)
          (Rendering|Material|SetVectorParameterValue _flashmat "FlashVector" (Math|Conversions|ToLinearColor(Vector) (Math|Vector|MakeVector 0.0 0.0 0.0)) :!class /Script/Engine.MaterialInstanceDynamic))
        (:then_1
          (bind _newtrack_1 (Timeline|Shake PlayFromStart)
            (:Update
              (CallFunction|SetObstacleScale _newtrack_1))))))
    (:then_1
      (Utilities|IsValid _hitsound
        (:Is%20Valid
          (Utilities|IsValid _barricade
            (:Is%20Valid
              (Audio|PlaySoundatLocation _hitsound (Transformation|GetWorldLocation _barricade) "0, 0, 0" 1.0 1.0 0.0 0 0 0 0))))))
    (:then_2
      (bind _opaciity (Timeline|Timeline PlayFromStart)
        (:Update
          (Utilities|IsValid _returnvalue
            (:Is%20Valid
              (bind _aswb_health_bar (Utilities|Casting|CastToWB_HealthBar _returnvalue))
              (Default|SetOpacity _aswb_health_bar _opaciity))))
        (:Finished
          (Variables|Default|SethealthBarVisible false))))))

(event EventObstacleDestroyed
  (bind _hb (Variables|Default|Gethb))
  (bind _destroysound (Variables|Default|GetDestroySound))
  (bind _returnvalue (UserInterface|GetWidget _hb))
  (Utilities|FlowControl|Sequence
    (:then_0
      (Effects|SpawnEmitteratLocation "/Game/VFX/Footing_Dust/P_ObstacleBreakPoof.P_ObstacleBreakPoof" (Transformation|GetWorldLocation (Variables|Default|GetBarricade))))
    (:then_1
      (Utilities|IsValid _destroysound
        (:Is%20Valid
          (Audio|PlaySoundatLocation _destroysound (Transformation|GetWorldLocation (Variables|Default|GetBarricade)) "0, 0, 0" 1.0 1.0 0.0 0 0 0 0))))
    (:then_2
      (bind _opaciity (Timeline|Timeline Stop)
        (:Update
          (Utilities|IsValid _returnvalue
            (:Is%20Valid
              (bind _aswb_health_bar (Utilities|Casting|CastToWB_HealthBar _returnvalue))
              (Default|SetOpacity _aswb_health_bar _opaciity))))
        (:Finished
          (Variables|Default|SethealthBarVisible false))))
    (:then_3
      (bind _newtrack_1 (Timeline|Shake Stop)
        (:Update
          (CallFunction|SetObstacleScale _newtrack_1))))
    (:then_4
      (Actor|DestroyActor))))

(event EventTick
  (params (DeltaSeconds :type Float%20%28single-precision%29))
  (if (Variables|Default|GethealthBarVisible)
    (CallFunction|HealthBarFaceCamera)))

(fn ConstructionScript)

(fn UpdateHealthBar
  (bind _aswb_health_bar (Utilities|Casting|CastToWB_HealthBar (UserInterface|GetWidget (Variables|Default|Gethb))))
  (Progress|SetPercent (Variables|/Game/Widgets/WB_HealthBar.WB_HealthBar_C|GetHealthBar _aswb_health_bar) (/ (Variables|Default|GetcurrentHealth) (Variables|Default|GetMaxObstacleHealth))))

(fn HealthBarFaceCamera
  (bind _hb (Variables|Default|Gethb))
  (bind _returnvalue (Transformation|GetWorldRotation _hb))
  (Transformation|SetWorldRotation _hb (Math|Rotator|MakeRotator (.roll _returnvalue) (.pitch _returnvalue) -1.8e+02) false false))

(fn ShowHealthBar
  (bind _aswb_health_bar (Utilities|Casting|CastToWB_HealthBar (UserInterface|GetWidget (Variables|Default|Gethb))))
  (bind _output_get (Variables|/Game/Widgets/WB_HealthBar.WB_HealthBar_C|SetOpaciity _aswb_health_bar 1.0)))

(fn SetFashMat
  (bind _barricade (Variables|Default|GetBarricade))
  (bind _returnvalue (Rendering|Material|CreateDynamicMaterialInstance _barricade 0 (Rendering|Material|GetMaterial _barricade 0) "FlashMat" :!class /Script/Engine.PrimitiveComponent))
  (bind _output_get (Variables|Default|SetFlashMat _returnvalue))
  (Rendering|Material|SetVectorParameterValue _output_get "FlashVector" (Math|Conversions|ToLinearColor(Vector) (Math|Vector|MakeVector 0.0 0.0 0.0)) :!class /Script/Engine.MaterialInstanceDynamic))

(fn SetObstacleScale
  (params (scale :type Float%20%28double-precision%29))
  (Transformation|SetWorldScale3D (Variables|Default|GetBarricade) (* (Variables|Default|GetScale) scale)))