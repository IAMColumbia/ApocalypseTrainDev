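; Spiked barrel obstacle that damages enemies and turns bloody when a knocked enemy hits it.
; A knocked enemy entering the box loses half its max health, swaps both meshes to the bloody material and plays a timeline that scales Cube from its initial size.
; Tick also deals small flat damage every frame to enemies overlapping Cube.
; Helper functions set up a dynamic flash material and rescale both meshes.
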(event OnComponentBeginOverlap(Box_0)
  (params (OverlappedComponent :type Primitive%20Component%20Object%20Reference) (OtherActor :type Actor%20Object%20Reference) (OtherComp :type Primitive%20Component%20Object%20Reference) (OtherBodyIndex :type Integer) (bFromSweep :type Boolean) (SweepResult :type Hit%20Result%20Structure%20%28by%20ref%29))
  (bind _asenemy_character (Utilities|Casting|CastToEnemyCharacter OtherActor))
  (Utilities|IsValid _asenemy_character
    (:Is%20Valid
      (if (Variables|/Script/Prototype0Unreal.EnemyCharacter|GetWasKnocked _asenemy_character)
        (Class|EnemyCharacter|TakeDamage _asenemy_character 0.0 (/ (Variables|/Script/Prototype0Unreal.EnemyCharacter|GetMaxHealth _asenemy_character) 2.0) "0, 0, 0" 0.0 false)
        (Rendering|Material|SetMaterial (Variables|Default|GetCube1) 0 "/Game/Models/SpikeTrapBLOODY_Mat.SpikeTrapBLOODY_Mat")
        (Rendering|Material|SetMaterial (Variables|Default|GetCube) 0 "/Game/Models/SpikeTrapBLOODY_Mat.SpikeTrapBLOODY_Mat")
        (bind _newtrack_1 (Timeline|Timeline_0 PlayFromStart)
          (:Update
            (Transformation|SetWorldScale3D (Variables|Default|GetCube) (* (Variables|Default|GetInitialScale) _newtrack_1))))))))

(event EventBeginPlay
  (bind _cube (Variables|Default|GetCube))
  (bind _returnvalue (Transformation|GetWorldScale _cube))
  (|CallParentFunction)
  (Variables|Default|SetInitialScale _returnvalue)
  (Variables|Default|SetScale _returnvalue))

(event Collision|EventActorBeginOverlap
  (params (OtherActor :type Actor%20Object%20Reference))
  (|CallParentFunction 0))

(event EventTick
  (params (DeltaSeconds :type Float%20%28single-precision%29))
  (bind _cube (Variables|Default|GetCube))
  (bind _overlappingactors (Collision|GetOverlappingActors _cube "/Game/Blueprints/Enemies/AI_Enemy.AI_Enemy_C" :!class /Script/Engine.PrimitiveComponent))
  (|CallParentFunction DeltaSeconds)
  (if (> (Utilities|Array|Length _overlappingactors) 0)
    (for _array_element _overlappingactors
      (bind _asenemy_character (Utilities|Casting|CastToEnemyCharacter _array_element))
      (Class|EnemyCharacter|TakeDamage _asenemy_character 0.0 5.0 "0, 0, 0" 0.0 false))))

(fn ConstructionScript)

(fn SetFashMat
  (bind _cube (Variables|Default|GetCube))
  (bind _returnvalue (Rendering|Material|CreateDynamicMaterialInstance _cube 0 (Rendering|Material|GetMaterial _cube 0) "FlashMat" :!class /Script/Engine.PrimitiveComponent))
  (bind _output_get (Variables|Default|SetFlashMat _returnvalue))
  (Rendering|Material|SetVectorParameterValue _output_get "FlashVector" (Math|Conversions|ToLinearColor(Vector) (Math|Vector|MakeVector 0.0 0.0 0.0)) :!class /Script/Engine.MaterialInstanceDynamic)
  (Rendering|Material|CreateDynamicMaterialInstance (Variables|Default|GetCube1) 0 _output_get "FlashMat" :!class /Script/Engine.PrimitiveComponent))

(fn SetObstacleScale
  (params (scale :type Float%20%28double-precision%29))
  (bind _cube (Variables|Default|GetCube))
  (Utilities|IsValid _cube
    (:Is%20Valid
      (Utilities|IsValid (Variables|Default|GetCube1)
        (:Is%20Valid
          (Transformation|SetWorldScale3D _cube (* (Variables|Default|GetScale) scale)))))))