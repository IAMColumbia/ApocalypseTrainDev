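; Tree obstacle that yields fuel as loot.
; Its DropLoot override runs the parent logic, then spawns a BP_FuelCollectable at the tree's location.
; The event graph holds only disabled placeholder events and the construction script just calls the parent, so all other behavior is inherited.
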(event EventBeginPlay
  (|CallParentFunction) ; This node is disabled and will not be called.\nDrag off pins to build functionality.
)

(event Collision|EventActorBeginOverlap
  (params (OtherActor :type Actor%20Object%20Reference))
  (|CallParentFunction OtherActor) ; This node is disabled and will not be called.\nDrag off pins to build functionality.
)

(event EventTick
  (params (DeltaSeconds :type Float%20%28single-precision%29))
  (|CallParentFunction DeltaSeconds) ; This node is disabled and will not be called.\nDrag off pins to build functionality.
)

(fn ConstructionScript
  (|CallParentFunction))

(fn DropLoot
  (|CallParentFunction)
  (Game|SpawnActorfromClass "/Game/Blueprints/BP_FuelCollectable.BP_FuelCollectable_C" (Math|Transform|MakeTransform (.location (Transformation|GetActorTransform)) "0, 0, 0" "1.000000,1.000000,1.000000") "Undefined" "MultiplyWithRoot" 0 0))