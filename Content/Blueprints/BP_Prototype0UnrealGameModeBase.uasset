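; Game mode for a local multiplayer prototype that creates players and gives each an input receiver pawn.
; On BeginPlay it gathers PlayerStarts and, for each index matching an integer PlayerStartTag, creates a player possessing a BP_InputReciever spawned at that array index's transform.
; SpawnPlayer later spawns and possesses a BP_MyCharacter at a receiver's transform.
; ChoosePlayerStart returns the first BP_CustomPlayerStart found for any player.
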(event Custom|SpawnPlayer_1_1
  (params (currentPlayerIndex :type Integer) (inputReciever :type BP%20Input%20Reciever%20Object%20Reference)))

(event EventBeginPlay
  (CallFunction|GetPlayerStartPoints)
  (CallFunction|SpawnInputRecievers))

(event EventTick
  (params (DeltaSeconds :type Float%20%28single-precision%29)))

(fn ConstructionScript)

(fn GetPlayerStartPoints
  (bind _outactors (Actor|GetAllActorsOfClass "/Script/Engine.PlayerStart"))
  (Variables|Default|SetPlayerStartArray _outactors))

(fn SpawnInputRecievers
  (for (_ _array_index) (Variables|Default|GetPlayerStartArray)
    (Variables|Default|SetIndex _array_index)
    (for _array_element (Variables|Default|GetPlayerStartArray)
      (if (== (CallFunction|NametoInt _array_element) (Variables|Default|GetIndex))
        (Class|GameplayStatics|CreatePlayer -1)
        (bind _returnvalue (Game|SpawnActorfromClass "/Game/Blueprints/BP_InputReciever.BP_InputReciever_C" (Transformation|GetActorTransform (Utilities|Array|Get(acopy) (Variables|Default|GetPlayerStartArray) (Variables|Default|GetIndex))) "Undefined" 0 (Variables|Default|GetIndex) 0))
        (Utilities|Array|AddUnique (Variables|Default|GetPlayerInputRecieverArray) _returnvalue)
        (Pawn|Possess (Game|GetPlayerController (Variables|Default|GetIndex)) _returnvalue)
        (Utilities|Array|AddUnique (Variables|Default|GetPlayerControllerArray) (Game|GetPlayerController (Variables|Default|GetIndex)))))))

(fn NametoInt
  (params (player%20start :type Player%20Start%20Object%20Reference))
  (return (Math|Conversions|ToInteger(Byte) (Utilities|String|ToString(Name) (Variables|/Script/Engine.PlayerStart|GetPlayerStartTag player%20start)))))

(fn ChoosePlayerStart
  (params (Player :type Controller%20Object%20Reference))
  (bind _returnvalue (Actor|GetActorOfClass "/Game/Blueprints/BP_CustomPlayerStart.BP_CustomPlayerStart_C"))
  (return _returnvalue))

(fn SpawnPlayer
  (params (currentPlayerIndex :type Integer) (inputReciever :type BP%20Input%20Reciever%20Object%20Reference))
  (Development|PrintString (Utilities|String|ToString(Integer) currentPlayerIndex))
  (bind _returnvalue (Game|SpawnActorfromClass "/Game/Blueprints/BP_MyCharacter.BP_MyCharacter_C" (Transformation|GetActorTransform inputReciever) "Undefined" (Game|GetPlayerController currentPlayerIndex) 0))
  (Pawn|Possess (Game|GetPlayerController currentPlayerIndex) _returnvalue)
  (return false))