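; BP_ChunkSpawner extends the level along the Y axis by spawning a chunk actor whenever SpawnLevelChunk is called.
; GetLevelChunk picks a random city or generic chunk, avoiding immediate repeats, and substitutes a train station at the encounter frequency.
; Each spawn advances YValue by chunk length, offsets NextTargetLocation to hide spawning, and moves the NavMeshBoundsVolume to the new chunk.
; An alternative PlaceChunk path repositioning existing chunks is never run.
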(event EventBeginPlay
  (bind _returnvalue (Actor|GetActorOfClass "/Script/NavigationSystem.NavMeshBoundsVolume"))
  (Variables|Default|SetNavMesh _returnvalue)
  (Variables|Default|SetTotalChunksSpawned 0))

(event Collision|EventActorBeginOverlap
  (params (OtherActor :type Actor%20Object%20Reference)))

(event EventSpawnLevelChunk
  (CallFunction|SpawnChunk))

(fn ConstructionScript)

(fn SpawnChunk
  (bind _output_get (Variables|Default|SetcurrentLocation (Math|Vector|MakeVector 0.0 (Variables|Default|GetyValue) 0.0)))
  (bind _chunktospawn (CallFunction|GetLevelChunk))
  (bind _returnvalue (Game|SpawnActorfromClass _chunktospawn (Math|Conversions|ToTransform(Vector) _output_get) "Undefined" "SelectDefaultAtRuntime" 0 0))
  (bind _length_out (Class|LevelChunk|GetLength _returnvalue))
  (bind _returnvalue_2 (Class|LevelChunk|GetScale _returnvalue))
  (Variables|Default|SetchunkScale _returnvalue_2)
  (Variables|Default|SetnextTargetLocation (- (Variables|Default|GetyValue) 6e+02))
  ;[1 1 1] RelocateNavmesh
  (Variables|Default|SetyValue (+ (Variables|Default|GetyValue) _length_out))
  (CallFunction|RelocateNavmesh _output_get)
  (Variables|Default|SetTotalChunksSpawned (+ (Variables|Default|GetTotalChunksSpawned) 1)))

(fn RelocateNavmesh
  (params (Location :type Vector))
  (bind _navmesh (Variables|Default|GetNavMesh))
  (Utilities|IsValid _navmesh
    (:Is%20Valid
      (Transformation|SetActorLocation _navmesh Location false false)
      (Class|NavigationSystemV1|OnNavigationBoundsUpdated (Class|NavigationSystemV1|GetNavigationSystem) _navmesh))
    (:Is%20Not%20Valid
      (Development|PrintString "NAVMESHNOTVALID"))))

(fn GetLevelChunk
  (bind _totalchunksspawned (Variables|Default|GetTotalChunksSpawned))
  (if (== _totalchunksspawned 0)
    _
    (elif (== (Math|Integer|%(Integer) _totalchunksspawned (Variables|Default|GetEncounterSpawnFrequency)) 0)
      (bind _output_get (LocalVariables|SetChunkClass "/Game/Blueprints/LevelChunks/BP_TrainStation.BP_TrainStation_C"))
      (return _output_get)
      (else
        _)))
  (Utilities|FlowControl|Sequence
    (:then_0
      (bind _output_get_2 (LocalVariables|SetChosenIndex (Math|Random|RandomInteger (Variables|Default|GetChunkVariations))))
      (if (== _output_get_2 (Variables|Default|GetPreviousChunkSpawned))
        (if (== (LocalVariables|GetChosenIndex) 0)
          (LocalVariables|SetChosenIndex (- (Variables|Default|GetChunkVariations) 1))
          (else
            (LocalVariables|SetChosenIndex (- (LocalVariables|GetChosenIndex) 1))))))
    (:then_1
      (switch int (LocalVariables|GetChosenIndex)
        (:Default
          (LocalVariables|SetChunkClass "/Game/Blueprints/BP_LevelChunk.BP_LevelChunk_C"))
        (:0
          (LocalVariables|SetChunkClass "/Game/Blueprints/LevelChunks/BP_Chunk6.BP_Chunk6_C"))
        (:1
          (LocalVariables|SetChunkClass "/Game/Blueprints/LevelChunks/BP_CityChunk1.BP_CityChunk1_C"))
        (:2
          (LocalVariables|SetChunkClass "/Game/Blueprints/LevelChunks/BP_CityChunk2.BP_CityChunk2_C"))
        (:3
          (LocalVariables|SetChunkClass "/Game/Blueprints/LevelChunks/BP_CityChunk3.BP_CityChunk3_C"))
        (:4
          (LocalVariables|SetChunkClass "/Game/Blueprints/LevelChunks/BP_CityChunk4.BP_CityChunk4_C"))
        (:5
          (LocalVariables|SetChunkClass "/Game/Blueprints/LevelChunks/BP_CityChunk5.BP_CityChunk5_C"))
        (:6
          (LocalVariables|SetChunkClass "/Game/Blueprints/LevelChunks/BP_Chunk7.BP_Chunk7_C"))))
    (:then_2
      (Variables|Default|SetPreviousChunkSpawned (LocalVariables|GetChosenIndex)))
    (:then_4
      (return (LocalVariables|GetChunkClass)))))

(fn PlaceChunk
  (bind _output_get (Variables|Default|SetcurrentLocation (Math|Vector|MakeVector 0.0 (Variables|Default|GetyValue) 0.0)))
  (bind _actor (CallFunction|GetChunktoMove))
  (Transformation|SetActorLocation _actor _output_get false false)
  (bind _length (Default|GetLengthBP _actor))
  (bind _scale (Default|GetScaleBP _actor))
  (Variables|Default|SetchunkScale _scale)
  (Variables|Default|SetnextTargetLocation (- (Variables|Default|GetyValue) 6e+02))
  ;[1 1 1] RelocateNavmesh
  (Variables|Default|SetyValue (+ (Variables|Default|GetyValue) _length))
  (CallFunction|RelocateNavmesh _output_get)
  (Variables|Default|SetTotalChunksSpawned (+ (Variables|Default|GetTotalChunksSpawned) 1)))

(fn GetChunktoMove
  (bind _output_get (LocalVariables|SetIntToSpawn (Math|Random|RandomInteger (Utilities|Array|Length (Variables|Default|GetLevelChunks)))))
  (if (or (== (Variables|Default|GetPreviousChunkSpawned) _output_get) (== (Variables|Default|GetPreviousPreviousChunkSpawned) _output_get))
    (if (== (LocalVariables|GetIntToSpawn) 0) :!label _label
      (bind _output_get_2 (LocalVariables|SetIntToSpawn (+ (LocalVariables|GetIntToSpawn) 1)))
      (if (== _output_get_2 (Variables|Default|GetPreviousPreviousChunkSpawned))
        (LocalVariables|SetIntToSpawn (+ (LocalVariables|GetIntToSpawn) 1))
        (else
          (Variables|Default|SetPreviousPreviousChunkSpawned (Variables|Default|GetPreviousChunkSpawned) :!label _label_2)
          (Variables|Default|SetPreviousChunkSpawned (LocalVariables|GetIntToSpawn))
          (return (Utilities|Array|Get(acopy) (Variables|Default|GetLevelChunks) (LocalVariables|GetIntToSpawn)))))
      (else
        (bind _output_get_3 (LocalVariables|SetIntToSpawn (- (LocalVariables|GetIntToSpawn) 1)))
        (if (== _output_get_3 (Variables|Default|GetPreviousPreviousChunkSpawned))
          (goto _label)
          (else
            (goto _label_2)))))
    (else
      (goto _label_2))))