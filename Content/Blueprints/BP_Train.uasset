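; The co-op game's player train: presents driving, fueling, impacts and game-over countdown through sound, VFX, materials and camera shake.
; Notify events drive that feedback, the turret vendor and HUD widgets for fuel, distance, critical warnings and per-player respawn timers.
; Tick updates the fuel bar, speed-based camera zoom, wheel spin, tutorial hints and custom-depth interactable highlights.
; Non-carried Fuel-tagged actors hitting the stockpile become fuel; purchased turrets attach to the holder.
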(event OnComponentHit(stockpile)
  (params (HitComponent :type Primitive%20Component%20Object%20Reference) (OtherActor :type Actor%20Object%20Reference) (OtherComp :type Primitive%20Component%20Object%20Reference) (NormalImpulse :type Vector :default "0, 0, 0") (Hit :type Hit%20Result%20Structure%20%28by%20ref%29))
  (CallFunction|DepositFuel OtherActor))

(event OnComponentBeginOverlap(CollisionDeposit)
  (params (OverlappedComponent :type Primitive%20Component%20Object%20Reference) (OtherActor :type Actor%20Object%20Reference) (OtherComp :type Primitive%20Component%20Object%20Reference) (OtherBodyIndex :type Integer) (bFromSweep :type Boolean) (SweepResult :type Hit%20Result%20Structure%20%28by%20ref%29)))

(event Custom|OnTurretPurchased_Event
  (bind _returnvalue (Game|SpawnActorfromClass "/Game/Blueprints/BP_TurretAttachment.BP_TurretAttachment_C" (Math|Transform|MakeTransform (Transformation|GetWorldLocation (Variables|Default|GetTurretHolder)) "0.000000,180.000000,0.000000" "1.000000,1.000000,1.000000") "AlwaysSpawn" "MultiplyWithRoot" self 0))
  (Transformation|AttachComponentToComponent _returnvalue (Variables|Default|GetTurretHolder) "None" "SnapToTarget" "KeepRelative" "KeepRelative" false)
  (Default|Deactivate (Variables|Default|GetTurretVendorReference)))

(event EventBeginPlay
  (Utilities|FlowControl|Sequence
    (:then_0
      (bind _returnvalue (Actor|GetActorOfClass "/Script/Engine.CameraActor"))
      (Utilities|IsValid (Actor|GetComponentbyClass _returnvalue "/Script/Engine.CameraComponent")
        (:Is%20Valid
          (bind _output_get (Variables|Default|SetMainCameraComponent (Actor|GetComponentbyClass _returnvalue "/Script/Engine.CameraComponent")))
          (Variables|Default|SetDefaultFOV (Variables|/Script/Engine.CameraComponent|GetFieldOfView _output_get))
          (bind _output_get_2 (Variables|Default|SetMainCameraActor _returnvalue))
          (Variables|Default|SetDefaultCamPos (Transformation|GetActorLocation _output_get_2)))))
    (:then_1
      (bind _returnvalue_2 (UserInterface|CreateWidget "/Game/Widgets/WB_TrainHealth.WB_TrainHealth_C"))
      (bind _output_get_3 (Variables|Default|SetFuelBar _returnvalue_2))
      (UserInterface|Viewport|AddtoViewport _output_get_3 0)
      (CallFunction|UpdateFuelBar))
    (:then_2
      (bind _returnvalue_3 (UserInterface|CreateWidget "/Game/Widgets/TotalMetersTraveled.TotalMetersTraveled_C"))
      (bind _output_get_4 (Variables|Default|SetMetersTraveled _returnvalue_3))
      (UserInterface|Viewport|AddtoViewport _output_get_4 0))
    (:then_3
      (bind _returnvalue_4 (UserInterface|CreateWidget "/Game/Widgets/WB_FuelCritical.WB_FuelCritical_C"))
      (bind _output_get_5 (Variables|Default|SetFuelCritical _returnvalue_4))
      (UserInterface|Viewport|AddtoViewport _output_get_5 0))
    (:then_4
      (Variables|Default|SetInitialNozzleScale (Transformation|GetWorldScale (Variables|Default|Getstockpile)))
      (Components|Activation|Deactivate (Variables|Default|GetFuelVFX)))
    (:then_5
      (bind _returnvalue_5 (Rendering|Material|CreateDynamicMaterialInstance (Variables|Default|Getstockpile) 0 "/Game/Mesh/TrainModelGameReady/TrainModelGameReady/GasNozzleMat.GasNozzleMat" "FlashMat" :!class /Script/Engine.PrimitiveComponent))
      (bind _output_get_6 (Variables|Default|SetFlashMat _returnvalue_5))
      (Rendering|Material|SetVectorParameterValue _output_get_6 "FlashVector" (Math|Conversions|ToLinearColor(Vector) (Math|Vector|MakeVector 0.0 0.0 0.0)) :!class /Script/Engine.MaterialInstanceDynamic))
    (:then_6
      (bind _returnvalue_6 (Actor|GetActorOfClass "/Game/Blueprints/LevelChunks/BP_TutorialChunk.BP_TutorialChunk_C"))
      (Variables|Default|SetTutorialChunk _returnvalue_6))
    (:then_7
      (bind _returnvalue_7 (Actor|GetActorOfClass "/Game/Blueprints/BP_MusicManager.BP_MusicManager_C"))
      (Variables|Default|SetMusicManager _returnvalue_7))
    (:then_8
      (EventDispatchers|BindEventtoTurretPurchased (Variables|Default|GetTurretVendorReference) (delegate Custom|OnTurretPurchased_Event))
      (Default|Deactivate (Variables|Default|GetTurretVendorReference)))
    (:then_9
      (CallFunction|SetupWheels))))

(event EventOnControllerPosses
  (params (PlayerIndex :type Integer) (playerColor :type Color%20Structure))
  (bind _widget (CallFunction|GetTimerbyIndex PlayerIndex))
  (CallFunction|SetupRespawnTimer _widget playerColor PlayerIndex)
  (Rendering|SetVisibility _widget false false)
  (Default|PlayerJoined (Variables|Default|GetFuelBar) playerColor))

(event EventNotifyTrainHitEnemy
  (Rendering|Material|SetMaterial (Variables|Default|GetTrainModelGameReady_SpikeFrontLOW_pCone7) 0 "/Game/Mesh/TrainModelGameReady/TrainModelGameReady/SpikesBloody.SpikesBloody"))

(event EventNotifyFuelCritical
  (bind _fuelcritical (Variables|Default|GetFuelCritical))
  (Rendering|Material|SetMaterial (Variables|Default|GetCube) 0 "/Game/Mesh/TrainModelGameReady/TrainModelGameReady/Button_Red.Button_Red")
  (Widget|SetVisibility (Variables|Default|GetFuelCritical) "Visible")
  (if (not (Variables|Default|GetplayingCritical))
    (Audio|PlaySound2D "/Game/Audio/AudioFiles/UI/FuelCriticalAlarm.FuelCriticalAlarm" 0.5 1.0 0.0 0 0)
    (Default|PlayPulse _fuelcritical)
    (bind _opaciy (Timeline|FlashCritical PlayFromStart)
      (:Update
        (Widget|SetRenderOpacity _fuelcritical _opaciy)
        (Variables|Default|SetplayingCritical true)
        (Rendering|SetVisibility (Variables|Default|GetFUELGOESHERE) true false))
      (:Finished
        (Variables|Default|SetplayingCritical false)))))

(event EventNotifyFuelNormal
  (Widget|SetVisibility (Variables|Default|GetFuelCritical) "Hidden")
  (Rendering|Material|SetMaterial (Variables|Default|GetCube) 0 "/Game/Mesh/TrainModelGameReady/TrainModelGameReady/button1.button1")
  (if (Variables|Default|GetCanMove)
    (Rendering|SetVisibility (Variables|Default|GetFUELGOESHERE) false false)))

(event EventNotifyTrainStart
  (bind _trainloopsound (Variables|Default|GetTrainLoopSound))
  (Utilities|FlowControl|Sequence
    (:then_0
      (Audio|SpawnSoundAttached "/Game/Audio/AudioFiles/Train/Train_Start.Train_Start" (Variables|Default|GetTrainModelGameReady_FrontHalfLOW_pCube23) "None" "0, 0, 0" "0, 0, 0" "KeepRelativeOffset" false 1.0 1.0 0.0 "/Game/Audio/BasicAttenuation.BasicAttenuation" 0)
      (Utilities|FlowControl|Delay 0.1)
      (Utilities|IsValid _trainloopsound
        (:Is%20Valid
          (Class|AudioComponent|SetPaused _trainloopsound false)
          (Components|Activation|Activate (Variables|Default|GetFuelVFX1) false))))
    (:then_1
      (Default|Deactivate (Variables|Default|GetTurretVendorReference)))))

(event EventNotifyTrainStop
  (bind _trainloopsound (Variables|Default|GetTrainLoopSound))
  (Utilities|FlowControl|Sequence
    (:then_0
      (Audio|SpawnSoundAttached "/Game/Audio/AudioFiles/Train/Train_Stop.Train_Stop" (Variables|Default|GetTrainModelGameReady_FrontHalfLOW_pCube23) "None" "0, 0, 0" "0, 0, 0" "KeepRelativeOffset" false 1.0 1.0 0.0 "/Game/Audio/BasicAttenuation.BasicAttenuation" 0)
      (Utilities|IsValid _trainloopsound
        (:Is%20Valid
          (Class|AudioComponent|SetPaused _trainloopsound true)
          (Components|Activation|Deactivate (Variables|Default|GetFuelVFX1)))))
    (:then_1
      (if (Utilities|Enum|Equal(Enum) (Variables|/Script/Prototype0Unreal.GameManagerWSS|GetCurrentGameState (Subsystems|GetGameManagerWSS)) "shopping")
        (Default|Activate (Variables|Default|GetTurretVendorReference))))))

(event EventNotifyTrainStartGame
  (Variables|Default|SetGameHasStarted true)
  (Audio|SpawnSoundAttached "/Game/Audio/AudioFiles/Train/Train_Start_Whistle.Train_Start_Whistle" (Variables|Default|GetTrainModelGameReady_FrontHalfLOW_pCube23) "None" "0, 0, 0" "0, 0, 0" "KeepRelativeOffset" false 1.0 1.0 0.0 "/Game/Audio/BasicAttenuation.BasicAttenuation" 0)
  (Utilities|FlowControl|Delay 0.1)
  (bind _returnvalue (Audio|SpawnSoundAttached "/Game/Audio/MetaSounds/Train_Source.Train_Source" (Variables|Default|GetTrainModelGameReady_FrontHalfLOW_pCube23) "None" "0, 0, 0" "0, 0, 0" "KeepRelativeOffset" false (Variables|Default|GetTrain%20Loop%20Volume) 1.0 0.0 "/Game/Audio/BasicAttenuation.BasicAttenuation" 0))
  (Variables|Default|SetTrainLoopSound _returnvalue)
  (Rendering|SetVisibility (Variables|Default|GetFUELGOESHERE) false false)
  (Default|FuelPickedUp (Variables|Default|GetTutorialChunk))
  (Default|TrainStarted (Variables|Default|GetFuelBar))
  (Default|PlayPickup (Variables|Default|GetMusicManager))
  (Components|Activation|Activate (Variables|Default|GetFuelVFX1) false))

(event EventNotifyFuelAdded
  (Audio|SpawnSoundAttached "/Game/Audio/MetaSounds/MS_FuelAddToTrain.MS_FuelAddToTrain" (Variables|Default|GetTrainModelGameReady_FrontHalfLOW_pCube23) "None" "0, 0, 0" "0, 0, 0" "KeepRelativeOffset" false 1.4 1.0 0.0 "/Game/Audio/BasicAttenuation.BasicAttenuation" 0)
  (Utilities|FlowControl|Sequence
    (:then_0
      (Rendering|Material|SetVectorParameterValue (Variables|Default|GetFlashMat) "FlashVector" (Math|Conversions|ToLinearColor(Vector) (Variables|Default|GetFlashColor)) :!class /Script/Engine.MaterialInstanceDynamic)
      (Utilities|FlowControl|Delay 0.2)
      (Rendering|Material|SetVectorParameterValue (Variables|Default|GetFlashMat) "FlashVector" (Math|Conversions|ToLinearColor(Vector) "0, 0, 0") :!class /Script/Engine.MaterialInstanceDynamic))
    (:then_1
      (bind _newtrack_1 (Timeline|Timeline_0 PlayFromStart)
        (:Update
          (Transformation|SetWorldScale3D (Variables|Default|Getstockpile) (* (Variables|Default|GetInitialNozzleScale) _newtrack_1)))))
    (:then_2
      (Utilities|FlowControl|Delay 0.2)
      (Components|Activation|Activate (Variables|Default|GetFuelVFX) false)
      (Utilities|FlowControl|Delay 0.5)
      (Components|Activation|Deactivate (Variables|Default|GetFuelVFX)))))

(event EventStartRespawnTimer
  (params (PlayerIndex :type Integer) (timeLeft :type Integer))
  ;[1 1 1] Respawn Timer
  (bind _widget (CallFunction|GetTimerbyIndex PlayerIndex))
  (CallFunction|UpdateTimerText _widget timeLeft)
  (Rendering|SetVisibility _widget true false))

(event EventUpdateTimer
  (params (PlayerIndex :type Integer) (timeLeft :type Integer))
  ;[1 1 1] Respawn Timer
  (bind _widget (CallFunction|GetTimerbyIndex PlayerIndex))
  (CallFunction|UpdateTimerText _widget timeLeft))

(event EventTick
  (params (DeltaSeconds :type Float%20%28single-precision%29))
  (bind _fueldeposit (Variables|Default|GetFuelDeposit))
  (Utilities|FlowControl|Sequence
    (:then_0
      (CallFunction|UpdateFuelBar)
      (CallFunction|UpdateCamerawithSpeed))
    (:then_1
      (CallFunction|UpdateInteractable (Variables|Default|GetstartTrainTrigger) (Variables|Default|GetCube) true))
    (:then_2
      (if (not (Variables|Default|GetGameHasStarted))
        (bind _returnvalue (Class|PlayerManagerWSS|AnyPlayerIsCarrying (Subsystems|GetPlayerManagerWSS)))
        (if _returnvalue
          (Rendering|SetVisibility (Variables|Default|GetFUELGOESHERE) true false)
          (Default|FuelPickedUp (Variables|Default|GetTutorialChunk))
          (else
            (Rendering|SetVisibility (Variables|Default|GetFUELGOESHERE) false false)
            (Default|NeedtoPickupFuel (Variables|Default|GetTutorialChunk))))))
    (:then_3
      (bind _returnvalue_2 (Class|PlayerManagerWSS|IsOverlappingPlayerwithFuel (Subsystems|GetPlayerManagerWSS) _fueldeposit))
      (CallFunction|UpdateInteractable _fueldeposit (Variables|Default|Getstockpile) _returnvalue_2))
    (:then_4
      (CallFunction|RotateWheels))))

(event EventStopRespawnTimer
  (params (PlayerIndex :type Integer) (timeLeft :type Integer))
  ;[1 1 1] Respawn Timer
  (bind _widget (CallFunction|GetTimerbyIndex PlayerIndex))
  (Rendering|SetVisibility _widget false false))

(event EventNotifyIncrementMeters
  (params (meters :type Integer))
  (Default|SetMetersTravelledText (Variables|Default|GetMetersTraveled) meters))

(event EventNotifyTrainHitObstacle
  (Default|PlayPusle (Variables|Default|GetFuelBar))
  (Camera|PlayWorldCameraShake "/Game/Blueprints/BP_CameraShake.BP_CameraShake_C" (Transformation|GetActorLocation) 0.0 2.5e+03)
  (Audio|SpawnSoundatLocation "/Game/Audio/MetaSounds/MS_TrainImpact.MS_TrainImpact" (Transformation|GetWorldLocation (Variables|Default|GetTrainModelGameReady_SpikeFrontLOW_pCone7)) "0, 0, 0" 1.0 1.0 0.0 0 0)
  (bind _outactors (Actor|GetAllActorsOfClass "/Game/Blueprints/BP_MyCharacter.BP_MyCharacter_C"))
  (for _array_element _outactors
    (Utilities|IsValid _array_element
      (:Is%20Valid
        (Game|Feedback|ClientPlayForceFeedback (Game|GetPlayerController (Variables|/Script/Prototype0Unreal.MyCharacter|GetPlayerIndex _array_element)) "/Game/FX/FF_TrainImpact.FF_TrainImpact" "None" false false false)))))

(event EventLeverStateChanged
  (CallFunction|UpdateLevers))

(event EventNotifyGameOverCounter
  (bind _gracetimeremaining (Variables|Default|GetGraceTimeRemaining))
  (bind _returnvalue (Game|SpawnActorfromClass "/Game/Widgets/BP_CountdownTextPopUp.BP_CountdownTextPopUp_C" (Transformation|GetWorldTransform (Variables|Default|GetGameOverTimer)) "Undefined" "OverrideRootScale" 0 0))
  (Default|SetupValuesasText _returnvalue (Utilities|Text|ToText(Integer) _gracetimeremaining) "(R=1.000000,G=1.000000,B=1.000000,A=1.000000)" 0.4)
  (Default|SetScale _returnvalue 1.0 1.0)
  (CallFunction|PlayCountdownSound _gracetimeremaining))

(fn ConstructionScript)

(fn UpdateFuelBar
  (Default|SetBarPercent (Variables|Default|GetFuelBar) (/ (Variables|Default|GetFuel) (Variables|Default|GetMaxFuel))))

(fn SetupRespawnTimer
  (params (Widget :type Widget%20Component%20Object%20Reference) (playercolor :type Color%20Structure) (playerindex :type Integer))
  (bind _asrespawn_timer (Utilities|Casting|CastToRespawnTimer (UserInterface|GetWidget Widget))
    (:then
      (Utilities|IsValid _asrespawn_timer
        (:Is%20Valid
          (Default|SetTimerColor _asrespawn_timer (Math|Conversions|ToLinearColor(Color) playercolor))
          (Default|SetTimerText _asrespawn_timer (Utilities|Text|ToText(Integer) playerindex)))))
    (:CastFailed
      (Development|PrintString "FAILED TO CAST TO WIDGET"))))

(fn GetTimerbyIndex
  (params (PlayerIndex :type Integer))
  (switch int PlayerIndex
    (:Default
      (LocalVariables|SetwidgetToReturn (Variables|Default|GetPlayer0RespawnTimer) :!label _label))
    (:0
      (goto _label))
    (:1
      (LocalVariables|SetwidgetToReturn (Variables|Default|GetPlayer1RespawnTimer)))
    (:2
      (LocalVariables|SetwidgetToReturn (Variables|Default|GetPlayer2RespawnTimer)))
    (:3
      (LocalVariables|SetwidgetToReturn (Variables|Default|GetPlayer3RespawnTimer))))
  (return (LocalVariables|GetwidgetToReturn)))

(fn UpdateTimerText
  (params (widget :type Widget%20Component%20Object%20Reference) (time :type Integer))
  (bind _asrespawn_timer (Utilities|Casting|CastToRespawnTimer (UserInterface|GetWidget widget)))
  (Default|SetTimerText _asrespawn_timer (Utilities|Text|ToText(Integer) time)))

(fn UpdateCamerawithSpeed
  (bind _maincameraactor (Variables|Default|GetMainCameraActor))
  (bind _maincameracomponent (Variables|Default|GetMainCameraComponent))
  (bind _currenttrainspeed (Variables|Default|GetcurrentTrainSpeed))
  (bind _returnvalue (Transformation|GetActorLocation _maincameraactor))
  (bind _returnvalue_2 (Math|Float|Absolute(Float) _currenttrainspeed))
  (if (Variables|Default|GetShouldZoomCamera)
    (Utilities|IsValid _maincameracomponent
      (:Is%20Valid
        (Camera|SetFieldOfView _maincameracomponent (+ (* _returnvalue_2 0.01) 9e+01))
        (Transformation|SetActorLocation _maincameraactor (Math|Vector|MakeVector (.x _returnvalue) (.y _returnvalue) (+ (.z (Variables|Default|GetDefaultCamPos)) (* _returnvalue_2 (Variables|Default|GetTrain%20Zoom%20Out)))) false false)))))

(fn UpdateInteractable
  (params (Trigger :type Box%20Component%20Object%20Reference%20%28by%20ref%29) (Mesh :type Static%20Mesh%20Component%20Object%20Reference%20%28by%20ref%29) (condition :type Boolean))
  (bind _returnvalue (Class|PlayerManagerWSS|IsOverlappingPlayer (Subsystems|GetPlayerManagerWSS) Trigger))
  (if _returnvalue
    (if condition
      (Rendering|SetRenderCustomDepth Mesh true)
      (for _array_element (Components|GetChildrenComponents Mesh false)
        (bind _asstatic_mesh_component (Utilities|Casting|CastToStaticMeshComponent _array_element))
        (Rendering|SetRenderCustomDepth _asstatic_mesh_component true)))
    (else
      (Rendering|SetRenderCustomDepth Mesh false)
      (for _array_element_2 (Components|GetChildrenComponents Mesh false)
        (bind _asstatic_mesh_component_2 (Utilities|Casting|CastToStaticMeshComponent _array_element_2))
        (Rendering|SetRenderCustomDepth _asstatic_mesh_component_2 false)))))

(fn UpdateLevers)

(fn GetBackBound
  (return (Variables|Default|GetBackBound)))

(fn PlayCountdownSound
  (params (time :type Integer))
  (Audio|PlaySound2D (Utilities|Array|Get(acopy) (LocalVariables|GetCountdownTime) time) 0.6 1.0 0.0 0 0))

(fn DepositFuel
  (params (Actor :type Actor%20Object%20Reference))
  (Utilities|IsValid Actor
    (:Is%20Valid
      (if (Actor|ActorHasTag Actor "Fuel")
        (bind _asinteractable_actor (Utilities|Casting|CastToInteractableActor Actor))
        (if (Utilities|Enum|NotEqual(Enum) (Variables|/Script/Prototype0Unreal.InteractableActor|Getstate _asinteractable_actor) "Carried")
          (bind _returnvalue (Class|Train|AddFuel))
          (if _returnvalue
            (Class|InteractableActor|OnFuelAddedtoTrain _asinteractable_actor)
            (Actor|DestroyActor Actor)))))))

(fn RotateWheels
  (for _array_element (Variables|Default|GetWheelList)
    (Transformation|SetWorldRotation _array_element (Math|Rotator|MakeRotator (+ (.roll (Transformation|GetWorldRotation _array_element)) (* (Variables|Default|GetcurrentTrainSpeed) (LocalVariables|GetWheelSpeedMultiplier))) 0.0 0.0) false false)))

(fn SetupWheels
  (Variables|Default|SetWheelList (Utilities|Array|MakeArray (Variables|Default|GetStaticMesh6) (Variables|Default|GetStaticMesh5) (Variables|Default|GetStaticMesh3) (Variables|Default|GetStaticMesh2) (Variables|Default|GetTrainWheelGameReady4) (Variables|Default|GetStaticMesh10) (Variables|Default|GetStaticMesh9) (Variables|Default|GetStaticMesh8) (Variables|Default|GetTrainWheelGameReady3) (Variables|Default|GetTrainWheelGameReady2) (Variables|Default|GetTrainWheelGameReady1) (Variables|Default|GetStaticMesh11))))