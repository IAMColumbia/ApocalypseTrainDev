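; Destructible barricade obstacle that shows its health and reacts visually when damaged.
; On damage it refreshes a widget health bar from current over maximum health.
; It also briefly flashes a dynamic material to white and plays a timeline that shakes the mesh by scaling its original world scale.
; A separate destroyed event removes the actor; health changes happen outside this graph.
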(event EventBeginPlay
  (CallFunction|UpdateHealthBar)
  (bind _returnvalue (Rendering|Material|CreateDynamicMaterialInstance (Variables|Default|GetBarricade) 0 "/Game/Mesh/StreetProps/Barricade2.Barricade2" "FlashMat" :!class /Script/Engine.PrimitiveComponent))
  (bind _output_get (Variables|Default|SetFlashMat _returnvalue))
  (Rendering|Material|SetVectorParameterValue _output_get "FlashVector" (Math|Conversions|ToLinearColor(Vector) (Math|Vector|MakeVector 0.0 0.0 0.0)) :!class /Script/Engine.MaterialInstanceDynamic)
  (Variables|Default|SetScale (Transformation|GetWorldScale (Variables|Default|GetBarricade))))

(event Collision|EventActorBeginOverlap
  (params (OtherActor :type Actor%20Object%20Reference)))

(event EventTick
  (params (DeltaSeconds :type Float%20%28single-precision%29)))

(event EventNotifyDamageObstacle
  (bind _flashmat (Variables|Default|GetFlashMat))
  (CallFunction|UpdateHealthBar)
  (Utilities|FlowControl|Sequence
    (:then_0
      (Rendering|Material|SetVectorParameterValue _flashmat "FlashVector" (Math|Conversions|ToLinearColor(Vector) (Math|Vector|MakeVector 1.0 1.0 1.0)) :!class /Script/Engine.MaterialInstanceDynamic)
      (Utilities|FlowControl|Delay 0.1)
      (Rendering|Material|SetVectorParameterValue _flashmat "FlashVector" (Math|Conversions|ToLinearColor(Vector) (Math|Vector|MakeVector 0.0 0.0 0.0)) :!class /Script/Engine.MaterialInstanceDynamic))
    (:then_1
      (bind _newtrack_1 (Timeline|Shake PlayFromStart)
        (:Update
          (Transformation|SetWorldScale3D (Variables|Default|GetBarricade) (* (Variables|Default|GetScale) _newtrack_1)))))))

(event EventObstacleDestroyed
  (Actor|DestroyActor))

(fn ConstructionScript)

(fn UpdateHealthBar
  (bind _aswb_health_bar (Utilities|Casting|CastToWB_HealthBar (UserInterface|GetWidget (Variables|Default|Gethb))))
  (Progress|SetPercent (Variables|/Game/Widgets/WB_HealthBar.WB_HealthBar_C|GetHealthBar _aswb_health_bar) (/ (Variables|Default|GetcurrentHealth) (Variables|Default|GetMaxObstacleHealth))))