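; BP_StatUpgrade is an interactable stat-upgrade crate with a red flare, outline highlight and prompt widget.
; Overlap events toggle the highlight and prompt, while BeginInteract pulses the mesh and advances OpenPercent, shown each Tick on a progress bar.
; Interacted spawns floating text from caller-supplied values, stops the flare, swaps to the opened mesh with a scale animation and sets Opened.
; Completion checks and stat changes are not handled here.
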(event EventBeginPlay
  (Utilities|Casting|CastToWB_HealthBar (UserInterface|GetWidget (Variables|Default|GetProgressBar)))
  (Effects|Components|ParticleSystem|SetColorParameter (Variables|Default|GetNS_FlareSmoke) "SmokeColor" "(R=1.000000,G=0.000000,B=0.065182,A=1.000000)")
  (Effects|Components|ParticleSystem|SetFloatParameter (Variables|Default|GetNS_FlareSmoke) "MaxLife" 5.0)
  (Variables|Default|SetInitialScale (Transformation|GetWorldScale (Variables|Default|GetCube)))
  (Rendering|SetVisibility (Variables|Default|GetProgressBar) false false)
  (Rendering|SetVisibility (Variables|Default|GetHldrb) false false))

(event Collision|EventActorBeginOverlap
  (params (OtherActor :type Actor%20Object%20Reference)))

(event EventTick
  (params (DeltaSeconds :type Float%20%28single-precision%29))
  (CallFunction|UpdateProgressBar))

(event EventPlayersOverlapping
  (Rendering|SetRenderCustomDepth (Variables|Default|GetCube) true)
  (if (not (Variables|Default|Getopened))
    (Rendering|SetVisibility (Variables|Default|GetHldrb) true false)))

(event EventNoPlayersOverlapping
  (Rendering|SetRenderCustomDepth (Variables|Default|GetCube) false)
  (Rendering|SetVisibility (Variables|Default|GetProgressBar) false false)
  (Rendering|SetVisibility (Variables|Default|GetHldrb) false false))

(event EventInteracted
  (params (textToDisplay :type Text%20%28by%20ref%29) (color :type Vector :default "0, 0, 0"))
  (Audio|SpawnSoundAttached "/Game/Audio/AudioFiles/LootCrateOpen.LootCrateOpen" (Variables|Default|GetCube) "None" "0, 0, 0" "0, 0, 0" "KeepRelativeOffset" false 1.0 (+ (Math|Random|RandomFloatinRange -0.1 0.1) 1.0) 0.0 "/Game/Audio/BasicAttenuation.BasicAttenuation" 0)
  (Utilities|FlowControl|Sequence
    (:then_0
      (bind _returnvalue (Game|SpawnActorfromClass "/Game/Widgets/BP_FloatingTextActor.BP_FloatingTextActor_C" (Math|Transform|MakeTransform (.location (Transformation|GetActorTransform)) "0, 0, 0" "1.000000,1.000000,1.000000") "Undefined" "OverrideRootScale" 0 0))
      (Default|SetupValuesasText _returnvalue textToDisplay (Math|Conversions|ToLinearColor(Vector) color) 0.3)
      (Default|SetScale _returnvalue 2.0 2.0)
      (Components|Activation|Deactivate (Variables|Default|GetNS_FlareSmoke))
      (Components|StaticMesh|SetStaticMesh (Variables|Default|GetCube) "/Game/Mesh/Interactables/AmmoBox/AmmoCrateOpened.AmmoCrateOpened")
      (bind _newtrack_1 (Timeline|Timeline_1 PlayFromStart)
        (:Update
          (Transformation|SetWorldScale3D (Variables|Default|GetCube) (* (Variables|Default|GetInitialScale) _newtrack_1))
          (Rendering|SetVisibility (Variables|Default|GetProgressBar) false false)
          (Rendering|SetVisibility (Variables|Default|GetHldrb) false false)
          (Variables|Default|Setopened true))))
    (:then_1
      (Rendering|SetVisibility (Variables|Default|GetProgressBar) false false))))

(event EventBeginInteract
  (Audio|SpawnSoundAttached "/Game/Audio/AudioFiles/LootCrateAttempt.LootCrateAttempt" (Variables|Default|GetCube) "None" "0, 0, 0" "0, 0, 0" "KeepRelativeOffset" false 1.0 (+ (Math|Random|RandomFloatinRange -0.1 0.1) 1.0) 0.0 "/Game/Audio/BasicAttenuation.BasicAttenuation" 0)
  (bind _newtrack_1 (Timeline|Timeline_0 PlayFromStart)
    (:Update
      (Transformation|SetWorldScale3D (Variables|Default|GetCube) (* (Variables|Default|GetInitialScale) _newtrack_1))
      (Rendering|SetVisibility (Variables|Default|GetProgressBar) true false)
      (Variables|Default|SetOpenPercent (+ (Variables|Default|GetOpenPercent) (* (Variables|Default|GetOpenRate) 2.0))))))

(fn ConstructionScript)

(fn UpdateProgressBar
  (bind _aswb_health_bar (Utilities|Casting|CastToWB_HealthBar (UserInterface|GetWidget (Variables|Default|GetProgressBar))))
  (Default|SetHealthPercent _aswb_health_bar (/ (Variables|Default|GetOpenPercent) (Variables|Default|GetOpenCompletePercent)))
  (Default|SetFillColor _aswb_health_bar (Variables|Default|GetProgressColor)))