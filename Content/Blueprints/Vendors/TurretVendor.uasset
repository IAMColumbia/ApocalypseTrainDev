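; Turret vendor actor that sells a turret, with a mesh, spotlight and price widget that appear only while it is active.
; Activate and Deactivate toggle CanBuy and those components' visibility, and Tick writes the item cost into the widget while CanBuy is set.
; Player overlap toggles a custom-depth highlight on the mesh until purchased.
; On purchase it sets the purchased flag, plays a sound and fires TurretPurchased.
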(event EventBeginPlay)

(event Collision|EventActorBeginOverlap
  (params (OtherActor :type Actor%20Object%20Reference)))

(event EventTick
  (params (DeltaSeconds :type Float%20%28single-precision%29))
  (if (Variables|Default|GetCanBuy)
    (bind _asvendor_info (Utilities|Casting|CastToVendorInfo (UserInterface|GetWidget (Variables|Default|GetInfo))))
    (Variables|/Game/Widgets/VendorInfo.VendorInfo_C|SetText _asvendor_info (Utilities|Text|ToText(Integer) (Variables|Default|GetCostOfItem)))))

(event EventPlayersOverlapping
  (if (not (Variables|Default|Gethaspurchased))
    (Rendering|SetRenderCustomDepth (Variables|Default|GetCube) true)))

(event EventNoPlayersOverlapping
  (Rendering|SetRenderCustomDepth (Variables|Default|GetCube) false))

(event EventOnPurchase
  (Variables|Default|Sethaspurchased true)
  (Audio|PlaySoundatLocation "/Game/Audio/MetaSounds/MS_Purchase.MS_Purchase" (Transformation|GetWorldLocation (Variables|Default|GetCube)) "0, 0, 0" 1.0 1.0 0.0 0 0 0 0)
  (Default|CallTurretPurchased))

(fn ConstructionScript)

(fn Deactivate
  (Variables|Default|SetCanBuy false)
  (Rendering|SetVisibility (Variables|Default|GetCube) false false)
  (Rendering|SetVisibility (Variables|Default|GetInfo) false false)
  (Rendering|SetVisibility (Variables|Default|GetSpotLight) false false))

(fn Activate
  (Variables|Default|SetCanBuy true)
  (Rendering|SetVisibility (Variables|Default|GetCube) true false)
  (Rendering|SetVisibility (Variables|Default|GetInfo) true false)
  (Rendering|SetVisibility (Variables|Default|GetSpotLight) true false))