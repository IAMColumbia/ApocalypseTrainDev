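; Weapon vendor actor that displays a purchasable gun as a looping, timeline-spun mesh with an info widget.
; BeginPlay sets mesh and scale from AvailableWeapon, while Tick fills the widget text, blanking it after purchase.
; Player overlap toggles a custom-depth highlight until bought, and purchase hides the gun and plays a sound.
; SetWeapon, which filters weapons by players' loadouts and picks randomly, is not called in this graph.
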(event EventBeginPlay
  (CallFunction|SetMeshIcon)
  (Variables|Default|SetInitRot (Transformation|GetWorldRotation (Variables|Default|GetGunMesh)))
  (bind _rotation (Timeline|Timeline Play)
    (:Update
      (Transformation|SetWorldRotation (Variables|Default|GetGunMesh) (Math|Rotator|MakeRotator (.roll (Variables|Default|GetInitRot)) (.pitch (Variables|Default|GetInitRot)) (+ _rotation (.yaw (Variables|Default|GetInitRot)))) false false))
    (:Finished
      (Timeline|Timeline PlayFromStart))))

(event Collision|EventActorBeginOverlap
  (params (OtherActor :type Actor%20Object%20Reference)))

(event EventPlayersOverlapping
  (if (not (Variables|Default|GetHasPurchased))
    (Rendering|SetRenderCustomDepth (Variables|Default|GetGunMesh) true)))

(event EventNoPlayersOverlapping
  (Rendering|SetRenderCustomDepth (Variables|Default|GetGunMesh) false))

(event EventOnPurchase
  (Rendering|SetVisibility (Variables|Default|GetGunMesh) false false)
  (Audio|PlaySoundatLocation "/Game/Audio/MetaSounds/MS_Purchase.MS_Purchase" (Transformation|GetWorldLocation (Variables|Default|GetScene)) "0, 0, 0" 1.0 1.0 0.0 0 0 0 0))

(event EventTick
  (params (DeltaSeconds :type Float%20%28single-precision%29))
  (bind _asvendor_info (Utilities|Casting|CastToVendorInfo (UserInterface|GetWidget (Variables|Default|GetInfo))))
  (if (Variables|Default|GetHasPurchased)
    (Variables|/Game/Widgets/VendorInfo.VendorInfo_C|SetText _asvendor_info "")
    (else
      (Variables|/Game/Widgets/VendorInfo.VendorInfo_C|SetText _asvendor_info (Class|WeaponVendor|GetInfoText)))))

(fn ConstructionScript)

(fn SetWeapon
  (bind _returnvalue (Subsystems|GetPlayerManagerWSS))
  (Utilities|FlowControl|Sequence
    (:then_0
      (bind _returnvalue_2 (Class|PlayerManagerWSS|NumActivePlayers _returnvalue))
      (if (<= _returnvalue_2 0)
        (Utilities|Array|RemoveItem (Variables|Default|GetWeapons) "/Game/Blueprints/Weapons/BP_ARWeapon.BP_ARWeapon_C")))
    (:then_1
      (bind _returnvalue_3 (Class|PlayerManagerWSS|GetPlayerWeaponTypes _returnvalue))
      (for (_array_element _array_index) _returnvalue_3
        (if (== _array_index 0)
          (LocalVariables|Setweapon1 _array_element)
          (else
            (LocalVariables|SetAllPlayersHaveSameWeapon (== _array_element (LocalVariables|Getweapon1))))))
      (if (LocalVariables|GetAllPlayersHaveSameWeapon)
        (bind _returnvalue_4 (Utilities|Array|RemoveItem (Variables|Default|GetWeapons) (LocalVariables|Getweapon1)))
        (if _returnvalue_4
          (Development|PrintString "Removed Weapon")
          (else
            (Development|PrintString "NO!!!")))))
    (:then_2
      (Variables|Default|SetAvailableWeapon (.OutItem (Utilities|Array|Random (Variables|Default|GetWeapons)))))))

(fn SetMeshIcon
  (bind _gunmesh (Variables|Default|GetGunMesh))
  (bind _gunmesh_2 (Variables|Default|GetGunMesh))
  (bind _gunmesh_3 (Variables|Default|GetGunMesh))
  (bind _gunmesh_4 (Variables|Default|GetGunMesh))
  (Utilities|FlowControl|Sequence
    (:then_0
      (if (== (Variables|Default|GetAvailableWeapon) "/Game/Blueprints/Weapons/BP_ARWeapon.BP_ARWeapon_C")
        (Components|StaticMesh|SetStaticMesh _gunmesh_4 "/Game/Mesh/Weapons/AR_GameReadyNew.AR_GameReadyNew")
        (Transformation|SetWorldScale3D _gunmesh_4 "12.000000,12.000000,12.000000")))
    (:then_1
      (if (== (Variables|Default|GetAvailableWeapon) "/Game/Blueprints/Weapons/BP_LauncherWeapon.BP_LauncherWeapon_C")
        (Components|StaticMesh|SetStaticMesh _gunmesh "/Game/Mesh/Weapons/GrenadeLauncher/GrenadeLauncherGameReady.GrenadeLauncherGameReady")
        (Transformation|SetWorldScale3D _gunmesh "5.000000,5.000000,5.000000")))
    (:then_2
      (if (== (Variables|Default|GetAvailableWeapon) "/Game/Blueprints/Weapons/BP_SniperWeapon.BP_SniperWeapon_C")
        (Components|StaticMesh|SetStaticMesh _gunmesh_3 "/Game/Mesh/Weapons/SniperGameReadyFBX.SniperGameReadyFBX")
        (Transformation|SetWorldScale3D _gunmesh_3 "7.000000,7.000000,7.000000")))
    (:then_3
      (if (== (Variables|Default|GetAvailableWeapon) "/Game/Blueprints/Weapons/BP_ShotgunWeapon.BP_ShotgunWeapon_C")
        (Components|StaticMesh|SetStaticMesh _gunmesh_2 "/Game/Mesh/Weapons/ShotGun_GameReady.ShotGun_GameReady")
        (Transformation|SetWorldScale3D _gunmesh_2 "3.000000,3.000000,3.000000")))))