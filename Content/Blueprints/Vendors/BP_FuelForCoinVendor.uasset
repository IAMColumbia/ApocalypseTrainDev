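; Vendor actor that, on purchase, dispenses four BP_Coin actors at its dispense location, each with a small random horizontal offset.
; A timeline then animates the cube's scale relative to the scale captured at BeginPlay, and the Dispensing flag clears after a short delay once it finishes.
; Player overlap events toggle custom depth rendering on the cube.
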(event EventBeginPlay
  (Variables|Components|SetInitialScale (Transformation|GetWorldScale (Variables|Default|GetCube))))

(event Collision|EventActorBeginOverlap
  (params (OtherActor :type Actor%20Object%20Reference)))

(event EventTick
  (params (DeltaSeconds :type Float%20%28single-precision%29)))

(event EventOnPurchase
  (bind _returnvalue (Math|Random|RandomFloatinRange 0.0 1e+01))
  (bind _returnvalue_2 (Math|Random|RandomFloatinRange 0.0 1e+01))
  (bind _dispenselocation (Variables|Default|GetDispenseLocation))
  (bind _returnvalue_3 (Transformation|GetWorldLocation _dispenselocation))
  (bind _returnvalue_4 (+ _returnvalue_3 (Math|Vector|MakeVector _returnvalue_2 _returnvalue 0.0)))
  (Utilities|FlowControl|Sequence
    (:then_0
      (Game|SpawnActorfromClass "/Game/Blueprints/BP_Coin.BP_Coin_C" (Math|Transform|MakeTransform _returnvalue_4 "0, 0, 0" "1.000000,1.000000,1.000000") "Undefined" "MultiplyWithRoot" 0 0)
      (Game|SpawnActorfromClass "/Game/Blueprints/BP_Coin.BP_Coin_C" (Math|Transform|MakeTransform _returnvalue_4 "0, 0, 0" "1.000000,1.000000,1.000000") "Undefined" "MultiplyWithRoot" 0 0)
      (Game|SpawnActorfromClass "/Game/Blueprints/BP_Coin.BP_Coin_C" (Math|Transform|MakeTransform _returnvalue_4 "0, 0, 0" "1.000000,1.000000,1.000000") "Undefined" "MultiplyWithRoot" 0 0)
      (Game|SpawnActorfromClass "/Game/Blueprints/BP_Coin.BP_Coin_C" (Math|Transform|MakeTransform _returnvalue_4 "0, 0, 0" "1.000000,1.000000,1.000000") "Undefined" "MultiplyWithRoot" 0 0))
    (:then_1
      (bind _newtrack_1 (Timeline|Timeline PlayFromStart)
        (:Update
          (Transformation|SetWorldScale3D (Variables|Default|GetCube) (* _newtrack_1 (Variables|Components|GetInitialScale))))
        (:Finished
          (Utilities|FlowControl|Delay 1.8)
          (Variables|Default|SetDispensing false))))))

(event EventPlayersOverlapping
  (Rendering|SetRenderCustomDepth (Variables|Default|GetCube) true))

(event EventNoPlayersOverlapping
  (Rendering|SetRenderCustomDepth (Variables|Default|GetCube) false))

(fn ConstructionScript)