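; Fuel vendor that dispenses a BP_FuelCollectable at its dispense location on purchase and labels itself "4 - Fuel" through its info widget.
; Each purchase plays a timeline that scales the cube relative to its initial size, then clears the Dispensing flag after a short delay.
; Player overlap events toggle custom depth rendering on the cube, presumably for highlighting.
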(event EventBeginPlay
  (Variables|Default|SetInitialScale (Transformation|GetWorldScale (Variables|Default|GetCube)))
  (bind _asvendor_info (Utilities|Casting|CastToVendorInfo (UserInterface|GetWidget (Variables|Default|GetInfo))))
  (Variables|/Game/Widgets/VendorInfo.VendorInfo_C|SetText _asvendor_info "4 - Fuel"))

(event Collision|EventActorBeginOverlap
  (params (OtherActor :type Actor%20Object%20Reference)))

(event EventTick
  (params (DeltaSeconds :type Float%20%28single-precision%29)))

(event EventOnPurchase
  (Game|SpawnActorfromClass "/Game/Blueprints/BP_FuelCollectable.BP_FuelCollectable_C" (Math|Transform|MakeTransform (Transformation|GetWorldLocation (Variables|Default|GetDispenseLocation)) "0, 0, 0" "1.000000,1.000000,1.000000") "Undefined" "MultiplyWithRoot" 0 0)
  (bind _newtrack_1 (Timeline|Timeline PlayFromStart)
    (:Update
      (Transformation|SetWorldScale3D (Variables|Default|GetCube) (* _newtrack_1 (Variables|Default|GetInitialScale))))
    (:Finished
      (Utilities|FlowControl|Delay 1.8)
      (Variables|Default|SetDispensing false))))

(event EventPlayersOverlapping
  (Rendering|SetRenderCustomDepth (Variables|Default|GetCube) true))

(event EventNoPlayersOverlapping
  (Rendering|SetRenderCustomDepth (Variables|Default|GetCube) false))

(fn ConstructionScript)