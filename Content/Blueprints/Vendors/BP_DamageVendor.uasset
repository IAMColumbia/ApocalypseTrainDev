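; Damage vendor Blueprint that handles the visual feedback for an upgrade purchase station.
; Its VendorInfo widget is filled from GetInfoText on BeginPlay and every Tick, and player overlap toggles custom depth on the cube.
; A purchase plays a timeline that scales the cube from its initial size, then clears Dispensing after a delay.
; PurchasedUpgrade spawns colored floating text at the vendor's location.
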(event EventBeginPlay
  (Variables|Default|SetInitialScale (Transformation|GetWorldScale (Variables|Default|GetCube)))
  (bind _asvendor_info (Utilities|Casting|CastToVendorInfo (UserInterface|GetWidget (Variables|Default|GetInfo))))
  (Variables|/Game/Widgets/VendorInfo.VendorInfo_C|SetText _asvendor_info (Class|StatVendor|GetInfoText)))

(event Collision|EventActorBeginOverlap
  (params (OtherActor :type Actor%20Object%20Reference)))

(event EventOnPurchase
  (bind _newtrack_1 (Timeline|Timeline PlayFromStart)
    (:Update
      (Transformation|SetWorldScale3D (Variables|Default|GetCube) (* _newtrack_1 (Variables|Default|GetInitialScale))))
    (:Finished
      (Utilities|FlowControl|Delay 1.8)
      (Variables|Default|SetDispensing false))))

(event EventPlayersOverlapping
  (Rendering|SetRenderCustomDepth (Variables|Default|GetCube) true))

(event EventNoPlayersOverlapping
  (Rendering|SetRenderCustomDepth (Variables|Default|GetCube) false))

(event EventPurchasedUpgrade
  (params (textToDisplay :type Text%20%28by%20ref%29) (color :type Vector :default "0, 0, 0"))
  (bind _returnvalue (Game|SpawnActorfromClass "/Game/Widgets/BP_FloatingTextActor.BP_FloatingTextActor_C" (Math|Transform|MakeTransform (.location (Transformation|GetActorTransform)) "0, 0, 0" "1.000000,1.000000,1.000000") "Undefined" "OverrideRootScale" 0 0))
  (Default|SetupValuesasText _returnvalue textToDisplay (Math|Conversions|ToLinearColor(Vector) color) 0.3)
  (Default|SetScale _returnvalue 2.0 2.0))

(event EventTick
  (params (DeltaSeconds :type Float%20%28single-precision%29))
  (bind _asvendor_info (Utilities|Casting|CastToVendorInfo (UserInterface|GetWidget (Variables|Default|GetInfo))))
  (Variables|/Game/Widgets/VendorInfo.VendorInfo_C|SetText _asvendor_info (Class|StatVendor|GetInfoText)))

(fn ConstructionScript)