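; BP_MenuManager is an actor that manages the game over menu.
; On BeginPlay it creates a WB_GameOver widget, adds it to the viewport and keeps it hidden.
; GameOverNotify reveals the widget, switches the player to Game and UI input focused on it, then sets keyboard focus after a short delay.
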(event EventBeginPlay
  (bind _returnvalue (UserInterface|CreateWidget "/Game/Widgets/WB_GameOver.WB_GameOver_C"))
  (bind _output_get (Variables|Default|SetGameOverWidget _returnvalue))
  (UserInterface|Viewport|AddtoViewport _output_get 0)
  (Widget|SetVisibility (Variables|Default|GetGameOverWidget) "Hidden"))

(event Collision|EventActorBeginOverlap
  (params (OtherActor :type Actor%20Object%20Reference)))

(event EventTick
  (params (DeltaSeconds :type Float%20%28single-precision%29)))

(event EventGameOverNotify
  (params (GameOverReason :type Integer))
  (bind _gameoverwidget (Variables|Default|GetGameOverWidget))
  (Widget|SetVisibility _gameoverwidget "Visible")
  (Input|SetInputModeGameandUI (Game|GetPlayerController 0) _gameoverwidget "DoNotLock" true false)
  (Utilities|FlowControl|Delay 0.2)
  (Widget|SetKeyboardFocus _gameoverwidget))

(fn ConstructionScript)