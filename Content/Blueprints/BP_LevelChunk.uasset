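; BP_LevelChunk is a level segment Blueprint that exposes size queries and a random-removal helper, with no event or construction logic of its own.
; Its length comes from the Cube component's world Y scale times 100, and its scale from the Cube's world scale times ScaleMultiplier.
; RandomlyDestroy removes a valid component on a one-in-Odds roll, allowing variation between chunks.
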(event EventBeginPlay)

(event Collision|EventActorBeginOverlap
  (params (OtherActor :type Actor%20Object%20Reference)))

(event EventTick
  (params (DeltaSeconds :type Float%20%28single-precision%29)))

(fn ConstructionScript)

(fn GetLengthBP
  (bind _output_get (Variables|Default|SetLength (* (.Y (Math|Vector|BreakVector (Transformation|GetWorldScale (Variables|Default|GetCube)))) 1e+02)))
  (return _output_get))

(fn GetScaleBP
  (return (* (Transformation|GetWorldScale (Variables|Default|GetCube)) (LocalVariables|GetscaleMultiplier))))

(fn RandomlyDestroy
  (params (ActorToDestroy :type Child%20Actor%20Component%20Object%20Reference) (Odds :type Integer))
  (Utilities|IsValid ActorToDestroy
    (:Is%20Valid
      (switch int (Math|Random|RandomInteger Odds)
        (:0
          (Components|DestroyComponent ActorToDestroy))))))