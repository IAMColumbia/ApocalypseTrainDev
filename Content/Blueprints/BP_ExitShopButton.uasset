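; BP_ExitShopButton is an interactable button that lets players exit the shop by calling ExitStation on the game manager.
; Being picked up triggers the exit once, guarded by a WasPressed flag that this graph never resets.
; Player overlap events toggle custom depth rendering on the Cube to highlight the button while players are nearby.
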(event EventBeginPlay)

(event Collision|EventActorBeginOverlap
  (params (OtherActor :type Actor%20Object%20Reference)))

(event EventTick
  (params (DeltaSeconds :type Float%20%28single-precision%29)))

(event EventPlayersOverlapping
  (Rendering|SetRenderCustomDepth (Variables|Default|GetCube) true))

(event EventNoPlayersOverlapping
  (Rendering|SetRenderCustomDepth (Variables|Default|GetCube) false))

(event EventOnPickedUp
  (params (carrier :type Scene%20Component%20Object%20Reference))
  (if (not (Variables|Default|GetWasPressed))
    (Class|GameManagerWSS|ExitStation (Subsystems|GetGameManagerWSS))
    (Variables|Default|SetWasPressed true)))

(fn ConstructionScript)