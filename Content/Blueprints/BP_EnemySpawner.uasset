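; BP_EnemySpawner is an enemy spawner Blueprint, but its spawn logic is currently disconnected.
; BeginPlay sets only EnemiesPerChunk; NotifySpawnEnemy and the SpawnEnemy function entry are both empty.
; Unwired nodes would forward the notification to SpawnEnemy, spawn AI_Enemy at the given location, initialize its speed, health and damage, and optionally set its target.
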(event EventBeginPlay
  (Variables|Default|SetEnemiesPerChunk 4))

(event Collision|EventActorBeginOverlap
  (params (OtherActor :type Actor%20Object%20Reference)))

(event EventTick
  (params (DeltaSeconds :type Float%20%28single-precision%29)))

(event EventNotifySpawnEnemy
  (params (spawnLocation :type Vector :default "0, 0, 0") (rotation :type Rotator :default "0, 0, 0") (SetTarget :type Boolean) (target :type Vector :default "0, 0, 0")))

(fn ConstructionScript)

(fn SpawnEnemy
  (params (spawnLocation :type Vector) (rotation :type Rotator) (setTargetImediatly :type Boolean) (target :type Vector)))