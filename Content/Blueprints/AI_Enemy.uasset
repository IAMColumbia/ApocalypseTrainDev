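; Pooled melee enemy character that carries a socket-attached weapon and can be upgraded in health, damage and speed.
; Hits trigger a scale pulse, dynamic-material flash, blood and floating damage numbers, alert its AI controller and briefly slow it, while player dashes knock it back.
; Death disables weapon and collision, may drop train fuel with odds scaled by player count, then sinks the mesh before returning to the pool; respawning reverses the cleanup.
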(event OnComponentHit(CapsuleComponent)
  (params (HitComponent :type Primitive%20Component%20Object%20Reference) (OtherActor :type Actor%20Object%20Reference) (OtherComp :type Primitive%20Component%20Object%20Reference) (NormalImpulse :type Vector :default "0, 0, 0") (Hit :type Hit%20Result%20Structure%20%28by%20ref%29))
  (Utilities|FlowControl|Sequence
    (:then_0
      (if (not (Variables|Default|GetWasKnocked))
        (bind _asbp_my_character (Utilities|Casting|CastToBP_MyCharacter OtherActor))
        (Utilities|IsValid _asbp_my_character
          (:Is%20Valid
            (if (Variables|/Script/Prototype0Unreal.MyCharacter|GetisDashing _asbp_my_character)
              (Class|EnemyCharacter|Knockback (Math|Vector|Normalize (- (Transformation|GetActorLocation) (Transformation|GetActorLocation _asbp_my_character))) (Variables|/Game/Blueprints/BP_MyCharacter.BP_MyCharacter_C|GetDashKnockback _asbp_my_character))
              (Variables|Default|SetisDamaged true)
              (Utilities|FlowControl|Delay 0.3)
              (Variables|Default|SetisDamaged false))))))))

(event EventBeginPlay
  (bind _mesh (Variables|Character|GetMesh))
  (bind _returnvalue (Transformation|GetSocketTransform _mesh "WeaponSocketRight" "RTS_World"))
  (Utilities|FlowControl|Sequence
    (:then_0
      (bind _returnvalue_2 (Game|SpawnActorfromClass "/Game/Blueprints/Weapons/BP_EnemyWeapon.BP_EnemyWeapon_C" (Math|Transform|MakeTransform (.location _returnvalue) (.rotation _returnvalue) "0.200000,0.200000,0.200000") "Undefined" "OverrideRootScale" 0 0))
      (bind _output_get (Variables|Default|SetSpawnedWeapon _returnvalue_2))
      (Transformation|AttachComponentToComponent _output_get (Variables|Character|GetMesh) "WeaponSocketRight" "SnapToTarget" "SnapToTarget" "SnapToTarget" true))
    (:then_1
      (Rendering|SetCastShadow (Variables|Default|GetHealthBarWidget) false)
      (Variables|Default|SetInitialScale (Transformation|GetWorldScale (Variables|Character|GetMesh))))
    (:then_2
      (bind _returnvalue_3 (Rendering|Material|CreateDynamicMaterialInstance (Variables|Character|GetMesh) 0 "/Game/Mesh/Characters/lambert1.lambert1" "FlashMat" :!class /Script/Engine.PrimitiveComponent))
      (bind _output_get_2 (Variables|Default|SetFlashMat _returnvalue_3))
      (Rendering|Material|SetVectorParameterValue _output_get_2 "FlashVector" (Math|Conversions|ToLinearColor(Vector) (Math|Vector|MakeVector 0.0 0.0 0.0)) :!class /Script/Engine.MaterialInstanceDynamic))
    (:then_3
      (Variables|Default|SetDefaultMeshWorldLocation (Transformation|GetWorldLocation (Variables|Character|GetMesh))))))

(event EventNotifyHealthBarWidget
  (Utilities|FlowControl|Sequence
    (:then_0
      (bind _aswb_health_bar (Utilities|Casting|CastToWB_HealthBar (UserInterface|GetWidget (Variables|Default|GetHealthBarWidget))))
      (Progress|SetPercent (Variables|/Game/Widgets/WB_HealthBar.WB_HealthBar_C|GetHealthBar _aswb_health_bar) (/ (Variables|Default|GetcurrentHealth) (Variables|Default|GetMaxHealth))))
    (:then_1
      (Variables|/Script/Engine.CharacterMovementComponent|SetMaxWalkSpeed (Variables|Character|GetCharacterMovement) (Variables|Default|GetInjuredSpeed))
      (Utilities|FlowControl|Delay 0.2)
      (Variables|/Script/Engine.CharacterMovementComponent|SetMaxWalkSpeed (Variables|Character|GetCharacterMovement) (Variables|Default|GetRunSpeed)))))

(event EventEnemyDespawned
  (bind _spawnedweapon (Variables|Default|GetSpawnedWeapon))
  (Utilities|IsValid _spawnedweapon
    (:Is%20Valid
      (if (Variables|/Game/Blueprints/Weapons/BP_EnemyWeapon.BP_EnemyWeapon_C|GetWeaponEnabled _spawnedweapon)
        (Variables|/Game/Blueprints/Weapons/BP_EnemyWeapon.BP_EnemyWeapon_C|SetWeaponEnabled _spawnedweapon false)))))

(event EventUpgradeEnemy
  (params (HealthIncrease :type Float%20%28single-precision%29) (DmgIncrease :type Float%20%28single-precision%29) (SpeedIncrease :type Float%20%28single-precision%29))
  (CallFunction|InitializeValues SpeedIncrease HealthIncrease DmgIncrease))

(event EventTick
  (params (DeltaSeconds :type Float%20%28single-precision%29))
  (Utilities|FlowControl|Sequence
    (:then_0
      (CallFunction|HealthBarFaceCamera))))

(event EventEnemySpawned
  (params (setTarget :type Boolean) (target :type Vector :default "0, 0, 0"))
  (Utilities|FlowControl|Sequence
    (:then_0
      (if setTarget
        (CallFunction|SetTarget target)))
    (:then_1
      (CallFunction|RespawnedCleanUp))))

(event EventMeleeAttack
  ;[1 1 1] Not in use
  (Variables|Default|SetisAttacking true))

(event EventSetAttackTarget
  (params (AttackTarget :type Actor%20Object%20Reference))
  (bind _returnvalue (Class|EnemyCharacter|IsinAttackRange AttackTarget))
  (if _returnvalue
    (if (not (Variables|Default|GetisAttacking))
      (Variables|Default|SetisAttacking true)
      (Utilities|FlowControl|Delay 2.0)
      (Variables|Default|SetisAttacking false))))

(event EventNotifyDamageEnemy
  (params (Damage :type Float%20%28single-precision%29))
  (Utilities|FlowControl|Sequence
    (:then_0
      (bind _newtrack_1 (Timeline|Pulse PlayFromStart)
        (:Update
          (Transformation|SetWorldScale3D (Variables|Character|GetMesh) (* (Variables|Default|GetInitialScale) _newtrack_1)))))
    (:then_1
      (bind _asmelee_enemy_controller (Utilities|Casting|CastToMeleeEnemyController (Pawn|GetController)))
      (if (not (Variables|/Game/AI/MeleeEnemyController.MeleeEnemyController_C|GetHasSensed _asmelee_enemy_controller))
        (Default|SetSensedTrue _asmelee_enemy_controller)))
    (:then_2
      (Components|Activation|Activate (Variables|Default|GetBlood) true))
    (:then_3
      (bind _returnvalue (Game|SpawnActorfromClass "/Game/Widgets/BP_FloatingTextActor.BP_FloatingTextActor_C" (Math|Transform|MakeTransform (+ (.location (Transformation|GetActorTransform)) (* (Math|Random|RandomUnitVector) "30.000000,30.000000,0")) "0, 0, 0" "1.000000,1.000000,1.000000") "Undefined" "OverrideRootScale" 0 0))
      (Default|SetupValues _returnvalue Damage 1.0))
    (:then_4
      (Variables|Default|SetisDamaged true)
      (Utilities|FlowControl|Delay 0.2)
      (Variables|Default|SetisDamaged false))
    (:then_5
      (Rendering|Material|SetVectorParameterValue (Variables|Default|GetFlashMat) "FlashVector" (Math|Conversions|ToLinearColor(Vector) (Variables|Default|GetFlashColor)) :!class /Script/Engine.MaterialInstanceDynamic)
      (Utilities|FlowControl|Delay (Variables|Default|GetFlashLength))
      (Rendering|Material|SetVectorParameterValue (Variables|Default|GetFlashMat) "FlashVector" (Math|Conversions|ToLinearColor(Vector) "0, 0, 0") :!class /Script/Engine.MaterialInstanceDynamic))))

(event EventActivateEnemy
  (Rendering|SetActorHiddenInGame (Variables|Default|GetSpawnedWeapon) false))

(event EventDeactivateEnemy
  (Rendering|SetActorHiddenInGame (Variables|Default|GetSpawnedWeapon) true))

(event EventEnemyKilled
  (bind _mesh (Variables|Character|GetMesh))
  (bind _returnvalue (Transformation|GetWorldLocation _mesh))
  (CallFunction|DeathCleanUp)
  (CallFunction|SpawnFuel)
  (Utilities|FlowControl|Delay 2.0)
  (bind _newtrack_0 (Timeline|MoveDown Play)
    (:Update
      (Transformation|SetWorldLocation (Variables|Character|GetMesh) (Math|Vector|MakeVector (.x _returnvalue) (.y _returnvalue) (+ (.z _returnvalue) (* _newtrack_0 (Variables|Default|GetSinkSpeed)))) false false))
    (:Finished
      (Class|PooledCharacter|DespawnPooledCharacter)
      (Transformation|SetWorldLocation (Variables|Character|GetMesh) (Variables|Default|GetDefaultMeshWorldLocation) false false))))

(fn ConstructionScript)

(fn HealthBarFaceCamera
  (bind _healthbarwidget (Variables|Default|GetHealthBarWidget))
  (Transformation|SetWorldRotation _healthbarwidget (Math|Rotator|FindLookatRotation (Transformation|GetWorldLocation _healthbarwidget) (Transformation|GetWorldLocation (Variables|/Script/Engine.PlayerCameraManager|GetTransformComponent (Game|GetPlayerCameraManager 0)))) false false))

(fn SetCanDamage
  (params (canDamage :type Boolean))
  (bind _spawnedweapon (Variables|Default|GetSpawnedWeapon))
  (Utilities|IsValid _spawnedweapon
    (:Is%20Valid
      (Variables|/Game/Blueprints/Weapons/BP_EnemyWeapon.BP_EnemyWeapon_C|SetcanDamage _spawnedweapon canDamage))))

(fn SetTarget
  (params (targetLocation :type Vector))
  (bind _asmelee_enemy_controller (Utilities|Casting|CastToMeleeEnemyController (Pawn|GetController)))
  (Default|SetTargetLocation _asmelee_enemy_controller targetLocation))

(fn InitializeValues
  (params (Speed :type Float%20%28double-precision%29) (Health :type Float%20%28double-precision%29) (Damage :type Float%20%28double-precision%29))
  (bind _spawnedweapon (Variables|Default|GetSpawnedWeapon))
  (bind _output_get (Variables|Default|SetRunSpeed (+ (Math|Random|RandomFloatinRange 0.0 (Variables|Default|GetMaxRunModifier)) Speed)))
  (Variables|/Script/Engine.CharacterMovementComponent|SetMaxWalkSpeed (Variables|Character|GetCharacterMovement) _output_get)
  (bind _output_get_2 (Variables|Default|SetMaxHealth Health))
  (Variables|Default|SetcurrentHealth _output_get_2)
  (Utilities|IsValid _spawnedweapon
    (:Is%20Valid
      (Variables|/Game/Blueprints/Weapons/BP_EnemyWeapon.BP_EnemyWeapon_C|SetDamage _spawnedweapon Damage))
    (:Is%20Not%20Valid
      (Development|PrintString "SPAWNED WEAPON NULL"))))

(fn DeathCleanUp
  (bind _spawnedweapon (Variables|Default|GetSpawnedWeapon))
  (Utilities|FlowControl|Sequence
    (:then_0
      (Utilities|IsValid _spawnedweapon
        (:Is%20Valid
          (if (Variables|/Game/Blueprints/Weapons/BP_EnemyWeapon.BP_EnemyWeapon_C|GetWeaponEnabled _spawnedweapon)
            (Variables|/Game/Blueprints/Weapons/BP_EnemyWeapon.BP_EnemyWeapon_C|SetWeaponEnabled _spawnedweapon false)))))
    (:then_2
      (bind _asmelee_enemy_controller (Utilities|Casting|CastToMeleeEnemyController (AI|GetAIController self)))
      (Default|SettoDead _asmelee_enemy_controller))
    (:then_3
      (Collision|SetCollisionResponsetoChannel (Variables|Default|GetCapsuleComponent) "ECC_Pawn" "ECR_Ignore")
      (Collision|SetCollisionResponsetoChannel (Variables|Default|GetCapsuleComponent) "ECC_WorldDynamic" "ECR_Ignore")
      (Rendering|SetVisibility (Variables|Default|GetHealthBarWidget) false false))))

(fn SpawnFuel
  (bind _returnvalue (Class|PlayerManagerWSS|NumActivePlayers (Subsystems|GetPlayerManagerWSS)))
  (bind _returnvalue_2 (Class|GameManagerWSS|TrainFuelFull (Subsystems|GetGameManagerWSS)))
  (if (not _returnvalue_2)
    (switch int (Math|Random|RandomInteger (* _returnvalue 2))
      (:0
        (Game|SpawnActorfromClass "/Game/Blueprints/BP_FuelCollectable.BP_FuelCollectable_C" (Math|Transform|MakeTransform (.location (Transformation|GetActorTransform)) "0, 0, 0" "1.000000,1.000000,1.000000") "Undefined" "OverrideRootScale" 0 0)))))

(fn RespawnedCleanUp
  (bind _spawnedweapon (Variables|Default|GetSpawnedWeapon))
  (Utilities|FlowControl|Sequence
    (:then_0
      (Utilities|IsValid _spawnedweapon
        (:Is%20Valid
          (if (not (Variables|/Game/Blueprints/Weapons/BP_EnemyWeapon.BP_EnemyWeapon_C|GetWeaponEnabled _spawnedweapon))
            (Variables|/Game/Blueprints/Weapons/BP_EnemyWeapon.BP_EnemyWeapon_C|SetWeaponEnabled _spawnedweapon true)))))
    (:then_2
      (bind _asmelee_enemy_controller (Utilities|Casting|CastToMeleeEnemyController (AI|GetAIController self)))
      (Default|SettoAlive _asmelee_enemy_controller))
    (:then_3
      (Collision|SetCollisionResponsetoChannel (Variables|Default|GetCapsuleComponent) "ECC_Pawn" "ECR_Block")
      (Collision|SetCollisionResponsetoChannel (Variables|Default|GetCapsuleComponent) "ECC_WorldDynamic" "ECR_Block")
      (Rendering|SetVisibility (Variables|Default|GetHealthBarWidget) true false))))

(fn GetAttackTarget
  (return 0))