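; BP_TrainStation is a train station piece that notifies the game manager as the train approaches and reaches the shop stop.
; Two overlap triggers respond only to components tagged Plow: EncounterStartTrigger calls ApproachingStation, and ShopTrainStopper calls EnterShop.
; It overrides GetLength to add the station floor's length, derived from its world Y scale, to the parent's length.
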(event OnComponentBeginOverlap(ShopTrainStopper)
  (params (OverlappedComponent :type Primitive%20Component%20Object%20Reference) (OtherActor :type Actor%20Object%20Reference) (OtherComp :type Primitive%20Component%20Object%20Reference) (OtherBodyIndex :type Integer) (bFromSweep :type Boolean) (SweepResult :type Hit%20Result%20Structure%20%28by%20ref%29))
  (if (Components|ComponentHasTag OtherComp "Plow")
    (Class|GameManagerWSS|EnterShop (Subsystems|GetGameManagerWSS))))

(event OnComponentBeginOverlap(EncounterStartTrigger)
  (params (OverlappedComponent :type Primitive%20Component%20Object%20Reference) (OtherActor :type Actor%20Object%20Reference) (OtherComp :type Primitive%20Component%20Object%20Reference) (OtherBodyIndex :type Integer) (bFromSweep :type Boolean) (SweepResult :type Hit%20Result%20Structure%20%28by%20ref%29))
  (if (Components|ComponentHasTag OtherComp "Plow")
    (Class|GameManagerWSS|ApproachingStation (Subsystems|GetGameManagerWSS))))

(event EventBeginPlay
  (|CallParentFunction) ; This node is disabled and will not be called.\nDrag off pins to build functionality.
)

(event Collision|EventActorBeginOverlap
  (params (OtherActor :type Actor%20Object%20Reference))
  (|CallParentFunction OtherActor) ; This node is disabled and will not be called.\nDrag off pins to build functionality.
)

(event EventTick
  (params (DeltaSeconds :type Float%20%28single-precision%29))
  (|CallParentFunction DeltaSeconds) ; This node is disabled and will not be called.\nDrag off pins to build functionality.
)

(fn ConstructionScript
  (|CallParentFunction))

(fn GetLength
  (bind _length_out (|CallParentFunction))
  (return (+ (* (.y (Transformation|GetWorldScale (Variables|Default|Getstation%20floor))) 1e+02) _length_out)))