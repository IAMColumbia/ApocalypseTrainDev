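; Player character for up to four local players, handling per-player colors, UI and feedback.
; Possession sets up the tinted indicator circle, player material and HUD widget.
; Notify events drive timeline scale pulses, flash-material hits, force feedback, dash effects, shooting speed changes, and death or respawn toggling of visibility, collision, input and AI stimuli.
; Upgrades raise damage, health or speed, while Tick refreshes health bars and the interact prompt.
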(event EventBeginPlay
  (Utilities|FlowControl|Sequence
    (:then_0
      (Variables|Default|SetInitialScale (Transformation|GetWorldScale (Variables|Default|GetcharacterMesh))))
    (:then_1
      (Rendering|SetCastShadow (Variables|Default|GetHealthBarWidget) false))
    (:then_2
      (bind _returnvalue (UserInterface|CreateWidget "/Game/Widgets/Bounds.Bounds_C"))
      (Variables|Default|SetBoundsWidgetREF _returnvalue)
      (CallFunction|RespawnPlayer))
    (:then_3
      (Components|Activation|Activate (Variables|Default|GetBulletTrails) false))
    (:then_4
      (Variables|Default|SetCircleInitalScale (Transformation|GetWorldScale (Variables|Default|GetPlayerCircle))))
    (:then_5
      (Variables|Default|SetBaseMaxRunSpeed (Variables|Default|GetMaxRunSpeed)))))

(event Collision|EventActorBeginOverlap
  (params (OtherActor :type Actor%20Object%20Reference)))

(event EventNotifyStoppedShooting
  ;[1 1 1] Bullet Particle Spawning
  (Variables|/Script/Engine.CharacterMovementComponent|SetMaxWalkSpeed (Variables|Character|GetCharacterMovement) (Variables|Default|GetMaxRunSpeed)))

(event EventNotifyPlayerDied
  (CallFunction|KillPlayer)
  (Variables|Default|SetMaxRunSpeed (Variables|Default|GetBaseMaxRunSpeed)))

(event EventNotifyonDash
  (params (direction :type Vector :default "0, 0, 0"))
  ;[1 1 1] Dash
  (Effects|SpawnEmitteratLocation "/Game/VFX/Footing_Dust/P_FootPoof_Dash.P_FootPoof_Dash" (Transformation|GetSocketLocation (Variables|Default|GetcharacterMesh) "None"))
  (Audio|SpawnSoundAttached "/Game/Audio/AudioFiles/Dash.Dash" (Variables|Default|GetcharacterMesh) "None" "0, 0, 0" "0, 0, 0" "KeepRelativeOffset" false 0.4 (+ (Math|Random|RandomFloatinRange -0.1 0.1) 1.0) 0.0 "/Game/Audio/BasicAttenuation.BasicAttenuation" 0)
  (bind _newtrack_1 (Timeline|Timeline_1 PlayFromStart)
    (:Update
      (Transformation|SetWorldScale3D (Variables|Default|GetPlayerCircle) (* (Variables|Default|GetCircleInitalScale) _newtrack_1)))))

(event EventNotifyReloadPercent
  (params (currentTime :type Float%20%28single-precision%29) (MaxTime :type Float%20%28single-precision%29))
  (bind _aswb_reload_bar (Utilities|Casting|CastToWB_reloadBar (UserInterface|GetWidget (Variables|Default|GetReloadBarWidget))))
  (Default|SetReloadPercent _aswb_reload_bar (/ currentTime MaxTime)))

(event EventOnDashFinish
  ;[1 1 1] Dash
)

(event EventNotifyWeaponEquipped
  (params (weaponNum :type Integer))
  (bind _playerui (Variables|Default|GetPlayerUI))
  (Utilities|IsValid _playerui
    (:Is%20Valid
      (Default|SetWeaponTexture _playerui weaponNum))))

(event EventNotifyShot
  (Variables|Default|SetShotFired true))

(event EventUpdateCoinUI
  (Default|UpdateCoinValue (Variables|Default|GetPlayerUI) (Variables|Default|GetCoins))
  (Game|Feedback|ClientPlayForceFeedback (Game|GetPlayerController (Variables|Default|GetPlayerIndex)) "/Game/FX/FF_CoinPickup.FF_CoinPickup" "None" false false false)
  (Utilities|FlowControl|Sequence
    (:then_0
      (bind _newtrack_1 (Timeline|Timeline_4 PlayFromStart)
        (:Update
          (Transformation|SetWorldScale3D (Variables|Default|GetcharacterMesh) (* (Variables|Default|GetInitialScale) _newtrack_1)))))))

(event EventTick
  (params (DeltaSeconds :type Float%20%28single-precision%29))
  (CallFunction|UpdateInteractUI)
  (CallFunction|UpdateHealthBar))

(event EventPossessed
  (params (NewController :type Controller%20Object%20Reference))
  (bind _playercolor (Variables|Default|GetPlayerColor))
  ;[1 1 1] Setup Indicators
  (Utilities|FlowControl|Sequence
    (:then_0
      (Class|MyCharacter|OnPlayerSpawn)
      (bind _returnvalue (Rendering|Material|CreateDynamicMaterialInstance "/Game/Materials/IndicatorMaterial.IndicatorMaterial" "instance" "Transient" :!class /Script/Engine.KismetMaterialLibrary))
      (Rendering|Material|SetMaterial (Variables|Default|GetPlayerCircle) (Variables|Default|GetPlayerIndex) _returnvalue)
      (Rendering|Material|SetVectorParameterValueonMaterials (Variables|Default|GetPlayerCircle) "BaseColor" _playercolor)
      ;[1 1 1] Set Health bar fill color
      (bind _aswb_health_bar (Utilities|Casting|CastToWB_HealthBar (UserInterface|GetWidget (Variables|Default|GetHealthBarWidget))))
      (Default|SetFillColor _aswb_health_bar (Variables|Default|GetPlayerColor)))
    (:then_1
      (bind _newparam (CallFunction|SetPlayerTexture (Variables|Default|GetPlayerIndex)))
      ;[1 1 1] Create Flash Material
      (bind _returnvalue_2 (Rendering|Material|CreateDynamicMaterialInstance (Variables|Character|GetMesh) 0 _newparam "FlashMat" :!class /Script/Engine.PrimitiveComponent))
      (bind _output_get (Variables|Components|SetFlashMat _returnvalue_2))
      (Rendering|Material|SetVectorParameterValue _output_get "FlashVector" (Math|Conversions|ToLinearColor(Vector) (Math|Vector|MakeVector 0.0 0.0 0.0)) :!class /Script/Engine.MaterialInstanceDynamic)
      ;;[1 1 1] Setup PlayerUI widget
      (bind _returnvalue_3 (UserInterface|CreateWidget "/Game/Widgets/PlayerUI_Widget.PlayerUI_Widget_C" (Game|GetPlayerController (Variables|Default|GetPlayerIndex))))
      (bind _output_get_2 (Variables|Default|SetPlayerUI _returnvalue_3))
      (UserInterface|Viewport|AddtoViewport _output_get_2 0)
      (Default|SetPlayerColor _output_get_2 _playercolor)
      (CallFunction|SetUILocation)
      (CallFunction|UpdateHealthBar))))

(event EventNotifyHealthBarWidget
  ;[1 1 1] Update Health Bar
  (CallFunction|UpdateHealthBar))

(event EventApplyUpgrade
  (params (upgrade :type EUpgradeType%20Enum :default "damage") (amount :type Float%20%28single-precision%29))
  (Utilities|FlowControl|Sequence
    (:then_0
      (Rendering|Material|SetVectorParameterValue (Variables|Components|GetFlashMat) "FlashVector" (Math|Conversions|ToLinearColor(Vector) (Variables|Default|GetPlayerColor)) :!class /Script/Engine.MaterialInstanceDynamic)
      (Utilities|FlowControl|Delay 0.4)
      (Rendering|Material|SetVectorParameterValue (Variables|Components|GetFlashMat) "FlashVector" (Math|Conversions|ToLinearColor(Vector) "0, 0, 0") :!class /Script/Engine.MaterialInstanceDynamic))
    (:then_1
      (switch Utilities|FlowControl|Switch|SwitchonEUpgradeType upgrade
        (:damage
          (Variables|Default|SetDamageBuff (+ (Variables|Default|GetDamageBuff) amount)))
        (:health
          (Variables|Default|SetMaxHealth (+ (Variables|Default|GetMaxHealth) amount))
          (CallFunction|UpdateHealthBar)
          (Class|MyCharacter|Heal))
        (:speed
          (bind _output_get (Variables|Default|SetSpeedBuff (+ (Variables|Default|GetSpeedBuff) amount)))
          (Variables|Default|SetMaxRunSpeed (+ _output_get (Variables|Default|GetMaxRunSpeed))))))))

(event EventNotifyFiredShot
  (params (direction :type Vector :default "0, 0, 0"))
  ;[1 1 1] Old Shooting VFX code (Not Used)
  (Effects|Components|ParticleSystem|SetVectorParameter (Variables|Default|GetBulletTrails) "user.ParticleDirection" (* direction (Variables|Default|GetBulletVelocity)))
  (Game|Feedback|ClientPlayForceFeedback (Game|GetPlayerController (Variables|Default|GetPlayerIndex)) "/Game/FX/FF_Shoot.FF_Shoot" "None" false false false))

(event EventNotifyPlayerRespawn
  (CallFunction|RespawnPlayer))

(event EventNotifyTakeDamage
  (Game|Feedback|ClientPlayForceFeedback (Game|GetPlayerController (Variables|Default|GetPlayerIndex)) "/Game/FX/FF_PlayerDamage.FF_PlayerDamage" "None" false false false)
  (Utilities|FlowControl|Sequence
    (:then_0
      (bind _newtrack_1 (Timeline|Timeline_0 PlayFromStart)
        (:Update
          (Transformation|SetWorldScale3D (Variables|Default|GetcharacterMesh) (* (Variables|Default|GetInitialScale) _newtrack_1)))))
    (:then_1
      (bind _newtrack_1_2 (Timeline|Timeline_2 PlayFromStart)
        (:Update
          (Transformation|SetWorldScale3D (Variables|Default|GetPlayerCircle) (* (Variables|Default|GetCircleInitalScale) _newtrack_1_2)))))
    (:then_2
      (Rendering|Material|SetVectorParameterValue (Variables|Components|GetFlashMat) "FlashVector" (Math|Conversions|ToLinearColor(Vector) (Variables|Default|GetFlashColor)) :!class /Script/Engine.MaterialInstanceDynamic)
      (Utilities|FlowControl|Delay 0.2)
      (Rendering|Material|SetVectorParameterValue (Variables|Components|GetFlashMat) "FlashVector" (Math|Conversions|ToLinearColor(Vector) "0, 0, 0") :!class /Script/Engine.MaterialInstanceDynamic))))

(event EventNotifyStartedShooting
  ;[1 1 1] Bullet Particle Spawning
  (Variables|/Script/Engine.CharacterMovementComponent|SetMaxWalkSpeed (Variables|Character|GetCharacterMovement) (Variables|Default|GetMaxShootingRunSpeed)))

(fn ConstructionScript)

(fn HealthBarFaceCamera
  (bind _healthbarwidget (Variables|Default|GetHealthBarWidget))
  (Transformation|SetWorldRotation _healthbarwidget (Math|Rotator|FindLookatRotation (Transformation|GetWorldLocation _healthbarwidget) (Transformation|GetWorldLocation (Variables|/Script/Engine.PlayerCameraManager|GetTransformComponent (Game|GetPlayerCameraManager 0)))) false false))

(fn RespawnPlayer
  (bind _playerindex (Variables|Default|GetPlayerIndex))
  (bind _returnvalue (Game|GetPlayerController _playerindex))
  (bind _returnvalue_2 (Game|GetPlayerCharacter _playerindex))
  (Rendering|SetVisibility (Variables|Default|GetcharacterMesh) true true)
  (Collision|SetCollisionEnabled (Variables|Default|GetCapsuleComponent) "QueryAndPhysics")
  (Utilities|IsValid _returnvalue_2
    (:Is%20Valid
      (Utilities|IsValid _returnvalue
        (:Is%20Valid
          (Input|EnableInput _returnvalue_2 _returnvalue)
          (Components|Activation|Activate (Variables|Default|GetAIPerceptionStimuliSource) false))))))

(fn KillPlayer
  (bind _playerindex (Variables|Default|GetPlayerIndex))
  (Components|Activation|Deactivate (Variables|Default|GetBulletTrails))
  (Variables|Default|SetIsShooting false)
  (Collision|SetCollisionEnabled (Variables|Default|GetCapsuleComponent) "NoCollision")
  (Rendering|SetVisibility (Variables|Default|GetcharacterMesh) false true)
  (Input|DisableInput (Game|GetPlayerCharacter _playerindex) (Game|GetPlayerController _playerindex))
  (Components|Activation|Deactivate (Variables|Default|GetAIPerceptionStimuliSource)))

(fn UpdateInteractUI
  (bind _interactwidget (Variables|Default|GetInteractWidget))
  (Rendering|SetVisibility (Variables|Default|GetInteractWidget) (Variables|Default|GetCanAddFuel) false)
  (Transformation|SetWorldRotation _interactwidget (Math|Rotator|FindLookatRotation (Transformation|GetWorldLocation _interactwidget) (Transformation|GetWorldLocation (Variables|/Script/Engine.PlayerCameraManager|GetTransformComponent (Game|GetPlayerCameraManager 0)))) false false))

(fn UpdateHealthBar
  (bind _playerui (Variables|Default|GetPlayerUI))
  (bind _aswb_health_bar (Utilities|Casting|CastToWB_HealthBar (UserInterface|GetWidget (Variables|Default|GetHealthBarWidget))))
  (Default|SetHealthPercent _aswb_health_bar (/ (Variables|Default|GetcurrentHealth) (Variables|Default|GetMaxHealth)))
  (Utilities|IsValid _playerui
    (:Is%20Valid
      (Default|SetHealthPercent _playerui (/ (Variables|Default|GetcurrentHealth) (Variables|Default|GetMaxHealth))))))

(fn IsDead
  (return (Variables|Default|GetIsPlayerDead)))

(fn SetPlayerTexture
  (params (index :type Integer))
  (Utilities|FlowControl|Sequence
    (:then_0
      (switch int index
        (:1
          (LocalVariables|Setmat "/Game/Mesh/Characters/player2_BaseColor_Mat.player2_BaseColor_Mat"))
        (:2
          (LocalVariables|Setmat "/Game/Mesh/Characters/player3_BaseColor_Mat.player3_BaseColor_Mat"))
        (:3
          (LocalVariables|Setmat "/Game/Mesh/Characters/player4_BaseColor_Mat.player4_BaseColor_Mat"))))
    (:then_1
      (return (LocalVariables|Getmat)))))

(fn SetUILocation
  (Utilities|FlowControl|Sequence
    (:then_0
      (switch int (Variables|Default|GetPlayerIndex)
        (:Default
          (LocalVariables|SetScreenPos "(X=-0.000000,Y=0.000000)"))
        (:0
          (LocalVariables|SetScreenPos "(X=200.000000,Y=1000.000000)"))
        (:1
          (LocalVariables|SetScreenPos "(X=800.000000,Y=1200.000000)"))
        (:2
          (LocalVariables|SetScreenPos "(X=1200.000000,Y=1200.000000)"))
        (:3
          (LocalVariables|SetScreenPos "(X=1600.000000,Y=1200.000000)"))))
    (:then_1
      (Class|UserWidget|SetPositioninViewport (Variables|Default|GetPlayerUI) (LocalVariables|GetScreenPos) true))))