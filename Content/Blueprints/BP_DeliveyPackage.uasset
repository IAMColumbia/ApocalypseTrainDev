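; BP_DeliveyPackage is a carryable physics package that players pick up and launch when dropped.
; It highlights the sphere through custom depth while players overlap.
; On pickup it stops simulating, snaps to the carrier's WeaponSocket and plays a randomly pitched sound.
; On drop it re-enables physics with an impulse; the first non-player hit returns it to Idle and plays a timeline scale animation on the sphere.
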(event OnComponentHit(Box)
  (params (HitComponent :type Primitive%20Component%20Object%20Reference) (OtherActor :type Actor%20Object%20Reference) (OtherComp :type Primitive%20Component%20Object%20Reference) (NormalImpulse :type Vector :default "0, 0, 0") (Hit :type Hit%20Result%20Structure%20%28by%20ref%29))
  (Utilities|IsValid OtherActor
    (:Is%20Valid
      (if (not (Actor|ActorHasTag OtherActor "Player"))
        (if (Variables|Default|GetwasDropped)
          (Variables|Default|SetwasDropped false)
          (Variables|Default|Setstate "Idle")
          (bind _newtrack_1 (Timeline|Timeline_0 PlayFromStart)
            (:Update
              (Transformation|SetWorldScale3D (Variables|Default|GetSphere) (* (Variables|Default|GetInitialScale) _newtrack_1)))))))))

(event EventBeginPlay
  (Variables|Default|SetInitialScale (Transformation|GetWorldScale (Variables|Default|GetSphere))))

(event Collision|EventActorBeginOverlap
  (params (OtherActor :type Actor%20Object%20Reference)))

(event EventTick
  (params (DeltaSeconds :type Float%20%28single-precision%29)))

(event EventPlayersOverlapping
  (Rendering|SetRenderCustomDepth (Variables|Default|GetSphere) true))

(event EventNoPlayersOverlapping
  (Rendering|SetRenderCustomDepth (Variables|Default|GetSphere) false))

(event EventOnPickedUp
  (params (carrier :type Scene%20Component%20Object%20Reference))
  (Physics|SetSimulatePhysics (Variables|Default|GetBox) false)
  (Transformation|AttachComponentToComponent carrier "WeaponSocket" "SnapToTarget" "SnapToTarget" "KeepWorld" true)
  (Audio|SpawnSoundAttached "/Game/Audio/MetaSounds/FuelPickup.FuelPickup" (Variables|Default|GetSphere) "None" "0, 0, 0" "0, 0, 0" "KeepRelativeOffset" false 1.4 (+ (Math|Random|RandomFloatinRange -0.1 0.1) 1.0) 0.0 "/Game/Audio/BasicAttenuation.BasicAttenuation" 0))

(event EventOnDropped
  (params (directionToLaunch :type Vector :default "0, 0, 0"))
  (bind _box (Variables|Default|GetBox))
  (Physics|SetSimulatePhysics _box true)
  (Physics|SetPhysicsLinearVelocity _box "0, 0, 0" false "None")
  (Physics|AddImpulse (Variables|Default|GetBox) (* directionToLaunch (Variables|Default|GetLaunchForce)) "None" false)
  (Variables|Default|SetwasDropped true))

(fn ConstructionScript)