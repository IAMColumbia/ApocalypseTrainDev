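; Coin pickup actor that scales in, spins and bobs in size, then flashes and destroys itself after its lifetime unless collected.
; Overlap by a living player disables physics and collision, plays a sound and a glowing scale pulse.
; Tick then homes it horizontally toward the player with accelerating speed, shrinking by normalized distance until it awards one coin.
; GoFlying launches the physics box in a random upward cone.
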(event OnComponentBeginOverlap(PickupRadius)
  (params (OverlappedComponent :type Primitive%20Component%20Object%20Reference) (OtherActor :type Actor%20Object%20Reference) (OtherComp :type Primitive%20Component%20Object%20Reference) (OtherBodyIndex :type Integer) (bFromSweep :type Boolean) (SweepResult :type Hit%20Result%20Structure%20%28by%20ref%29))
  (if (not (Variables|Default|GetPickedUp))
    (if (Actor|ActorHasTag OtherActor "Player")
      (bind _asmy_character (Utilities|Casting|CastToMyCharacter OtherActor))
      (bind _output_get (Variables|Default|SetOwnerCHaracter _asmy_character))
      (if (not (Variables|/Script/Prototype0Unreal.MyCharacter|GetIsPlayerDead _output_get))
        (Variables|Default|SetPickedUp true)
        (Physics|SetSimulatePhysics (Variables|Default|GetBox) false)
        (Collision|SetCollisionEnabled (Variables|Default|GetSphere) "NoCollision")
        (Audio|SpawnSoundatLocation "/Game/Audio/MetaSounds/Coin.Coin" (Transformation|GetActorLocation) "0, 0, 0" 1.0 1.0 0.0 0 0)
        (bind _scale (Timeline|Pulse PlayFromStart)
          (:Update
            (Transformation|SetWorldScale3D (Variables|Default|GetSphere) (* (Variables|Default|GetInitialSize) _scale))
            (Rendering|Material|SetScalarParameterValue (Variables|Default|GetFlashMat) "Emissive" (* (- _scale 1.0) 4.0) :!class /Script/Engine.MaterialInstanceDynamic))
          (:Finished
            (Variables|Default|SetMoveToPlayer true)
            (Variables|Default|SetmaxDis (Math|Vector|Distance(Vector) (Transformation|GetWorldLocation (Variables|Default|GetSphere)) (Transformation|GetWorldLocation (Variables|/Script/Prototype0Unreal.MyCharacter|GetcharacterMesh (Variables|Default|GetOwnerCHaracter)))))))))))

(event EventBeginPlay
  (bind _returnvalue (Rendering|Material|CreateDynamicMaterialInstance (Variables|Default|GetSphere) 0 "/Game/Mesh/Interactables/Newestcoin/CoinMat.CoinMat" "FlashMat" :!class /Script/Engine.PrimitiveComponent))
  (Variables|Default|SetFlashMat _returnvalue)
  (Variables|Default|SetInitialSize (Transformation|GetWorldScale (Variables|Default|GetSphere)))
  (Variables|Default|Setseconds (Math|Random|RandomFloatinRange 0.0 1.0))
  (Variables|Default|SetroatSpeed (Math|Random|RandomFloatinRange 0.8 1.2))
  (Transformation|AddLocalRotation (Variables|Default|GetSphere) (Math|Rotator|MakeRotator 0.0 0.0 (Math|Random|RandomFloatinRange 0.0 3.6e+02)) false false)
  (bind _scale (Timeline|Timeline PlayFromStart)
    (:Update
      (Transformation|SetWorldScale3D (Variables|Default|GetSphere) (* (Variables|Default|GetInitialSize) _scale))
      (Utilities|FlowControl|Delay (Variables|Default|GetLifeTime))
      (bind _opacity (Timeline|Flash PlayFromStart)
        (:Update
          (Rendering|Material|SetScalarParameterValue (Variables|Default|GetFlashMat) "Opacity" _opacity :!class /Script/Engine.MaterialInstanceDynamic))
        (:Finished
          (if (not (Variables|Default|GetPickedUp))
            (Actor|DestroyActor)))))))

(event EventTick
  (params (DeltaSeconds :type Float%20%28single-precision%29))
  (bind _ownercharacter (Variables|Default|GetOwnerCHaracter))
  (bind _sphere (Variables|Default|GetSphere))
  (bind _ownercharacter_2 (Variables|Default|GetOwnerCHaracter))
  (bind _sphere_2 (Variables|Default|GetSphere))
  (bind _output_get (Variables|Default|Setseconds (+ (Variables|Default|Getseconds) 1.0)))
  (if (Variables|Default|GetMoveToPlayer)
    (Utilities|IsValid _ownercharacter
      (:Is%20Valid
        (Transformation|SetWorldLocation _sphere (Math|Vector|MakeVector (.x (+ (* (- (Transformation|GetWorldLocation (Variables|/Script/Prototype0Unreal.MyCharacter|GetcharacterMesh _ownercharacter)) (Transformation|GetWorldLocation (Variables|Default|GetSphere))) (Variables|Default|GetMoveSpeed)) (Transformation|GetWorldLocation _sphere))) (.y (+ (* (- (Transformation|GetWorldLocation (Variables|/Script/Prototype0Unreal.MyCharacter|GetcharacterMesh _ownercharacter)) (Transformation|GetWorldLocation (Variables|Default|GetSphere))) (Variables|Default|GetMoveSpeed)) (Transformation|GetWorldLocation _sphere))) (.z (Transformation|GetWorldLocation (Variables|Default|GetSphere)))) false false)
        (Variables|Default|SetMoveSpeed (+ (Variables|Default|GetMoveSpeed) (Variables|Default|GetAcceleration)))
        (Transformation|SetWorldScale3D (Variables|Default|GetSphere) (* (Variables|Default|GetInitialSize) (CallFunction|NormalizeDistance)))
        (if (<= (CallFunction|NormalizeDistance) 0.1)
          (Utilities|IsValid _ownercharacter_2
            (:Is%20Valid
              (Class|MyCharacter|AddCoins _ownercharacter_2 1)
              (Variables|Default|SetMoveToPlayer false)
              (Actor|DestroyActor)))))
      (:Is%20Not%20Valid
        (Development|PrintString "player not valid - coin")))
    (elif (not (Variables|Default|GetPickedUp))
      (Transformation|AddLocalRotation _sphere_2 (Math|Rotator|MakeRotator 0.0 0.0 (Variables|Default|GetroatSpeed)) false false)
      (Transformation|SetWorldScale3D _sphere_2 (* (Variables|Default|GetInitialSize) (+ (* (Math|Trig|Sin(Radians) (* _output_get (Variables|Default|GetpusleFreq))) 0.1) 0.9))))))

(fn ConstructionScript)

(fn NormalizeDistance
  (bind _sphere (Variables|Default|GetSphere))
  (bind _ownercharacter (Variables|Default|GetOwnerCHaracter))
  (bind _returnvalue (Transformation|GetWorldLocation _sphere))
  (bind _charactermesh (Variables|/Script/Prototype0Unreal.MyCharacter|GetcharacterMesh _ownercharacter))
  (bind _returnvalue_2 (Transformation|GetWorldLocation _charactermesh))
  (Utilities|IsValid _ownercharacter
    (:Is%20Valid
      (return (/ (- (Math|Vector|Distance(Vector) (Math|Vector|MakeVector (.x _returnvalue) (.y _returnvalue) (.z _returnvalue)) (Math|Vector|MakeVector (.x _returnvalue_2) (.y _returnvalue_2) (.z _returnvalue))) (Variables|Default|GetminDis)) (- (Variables|Default|GetmaxDis) (Variables|Default|GetminDis)))))))

(fn GoFlying
  (Physics|AddImpulse (Variables|Default|GetBox) (* (Math|Random|RandomUnitVectorinConeinDegrees (Math|Vector|VectorUp) 5e+01) (Variables|Default|GetCoinLaunchForce)) "None" false))