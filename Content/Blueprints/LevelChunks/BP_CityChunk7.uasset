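; City level chunk variant that extends a parent chunk class and includes a hazard for the player.
; On BeginPlay it runs the parent logic, then calls RandomlyDestroy with fixed odds.
; Overlapping DeathCollision calls DespawnPlayer on the MyCharacter that entered it.
; GetLength adds the Y extents of Cube and TrainFloor, derived from world scale, to the parent's length.
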(event OnComponentBeginOverlap(DeathCollision)
  (params (OverlappedComponent :type Primitive%20Component%20Object%20Reference) (OtherActor :type Actor%20Object%20Reference) (OtherComp :type Primitive%20Component%20Object%20Reference) (OtherBodyIndex :type Integer) (bFromSweep :type Boolean) (SweepResult :type Hit%20Result%20Structure%20%28by%20ref%29))
  (bind _asmy_character (Utilities|Casting|CastToMyCharacter OtherActor))
  (Class|MyCharacter|DespawnPlayer _asmy_character 2.0))

(event EventBeginPlay
  (|CallParentFunction)
  (CallFunction|RandomlyDestroy 0 2))

(event Collision|EventActorBeginOverlap
  (params (OtherActor :type Actor%20Object%20Reference))
  (|CallParentFunction OtherActor) ; This node is disabled and will not be called.\nDrag off pins to build functionality.
)

(event EventTick
  (params (DeltaSeconds :type Float%20%28single-precision%29))
  (|CallParentFunction DeltaSeconds) ; This node is disabled and will not be called.\nDrag off pins to build functionality.
)

(fn ConstructionScript
  (|CallParentFunction))

(fn GetLength
  (bind _length_out (|CallParentFunction))
  (return (+ (+ _length_out (* (.Y (Math|Vector|BreakVector (Transformation|GetWorldScale (Variables|Default|GetCube)))) 1e+02)) (* (.Y (Math|Vector|BreakVector (Transformation|GetWorldScale (Variables|Default|GetTrainFloor)))) 1e+02))))