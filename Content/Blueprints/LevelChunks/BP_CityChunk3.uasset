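; BP_CityChunk3 is a city level chunk that extends a parent chunk Blueprint.
; On BeginPlay it runs the parent logic, then passes a placed fuel collectable to RandomlyDestroy, so that pickup's presence varies.
; GetLength adds the Y extents of the Cube and TrainFloor1 pieces to the parent's length, deriving each from world scale on a 100-unit base.
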(event EventBeginPlay
  (|CallParentFunction)
  (CallFunction|RandomlyDestroy (Variables|Default|GetBP_FuelCollectable7) 2))

(event Collision|EventActorBeginOverlap
  (params (OtherActor :type Actor%20Object%20Reference))
  (|CallParentFunction OtherActor) ; This node is disabled and will not be called.\nDrag off pins to build functionality.
)

(event EventTick
  (params (DeltaSeconds :type Float%20%28single-precision%29))
  (|CallParentFunction DeltaSeconds) ; This node is disabled and will not be called.\nDrag off pins to build functionality.
)

(fn ConstructionScript
  (|CallParentFunction))

(fn GetLength
  (bind _length_out (|CallParentFunction))
  (return (+ (+ _length_out (* (.Y (Math|Vector|BreakVector (Transformation|GetWorldScale (Variables|Default|GetCube)))) 1e+02)) (* (.Y (Math|Vector|BreakVector (Transformation|GetWorldScale (Variables|Default|GetTrainFloor1)))) 1e+02))))