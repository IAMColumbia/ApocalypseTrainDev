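; BP_TrainStation is a level chunk for a train station with a shop, reached after surviving a horde.
; Plow-tagged overlaps activate the station on approach and trigger shop entry through the game manager.
; While active, Tick opens entry doors on a manager flag and exit doors on a child-actor button press, then reports station entry or exit.
; Doors slide by a fixed per-frame step, and GetLength adds the floor's scaled length to the parent's.
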(event OnComponentBeginOverlap(ShopTrainStopper)
  (params (OverlappedComponent :type Primitive%20Component%20Object%20Reference) (OtherActor :type Actor%20Object%20Reference) (OtherComp :type Primitive%20Component%20Object%20Reference) (OtherBodyIndex :type Integer) (bFromSweep :type Boolean) (SweepResult :type Hit%20Result%20Structure%20%28by%20ref%29))
  (if (Components|ComponentHasTag OtherComp "Plow")
    (Class|GameManagerWSS|EnterShop (Subsystems|GetGameManagerWSS))))

(event OnComponentBeginOverlap(EncounterStartTrigger)
  (params (OverlappedComponent :type Primitive%20Component%20Object%20Reference) (OtherActor :type Actor%20Object%20Reference) (OtherComp :type Primitive%20Component%20Object%20Reference) (OtherBodyIndex :type Integer) (bFromSweep :type Boolean) (SweepResult :type Hit%20Result%20Structure%20%28by%20ref%29))
  (if (Components|ComponentHasTag OtherComp "Plow")
    (Class|GameManagerWSS|ApproachingStation (Subsystems|GetGameManagerWSS))
    (Variables|Default|SetCurrentlyActive true)
    (Development|PrintString "Survive The Horde!")))

(event EventBeginPlay
  (|CallParentFunction))

(event Collision|EventActorBeginOverlap
  (params (OtherActor :type Actor%20Object%20Reference))
  (|CallParentFunction OtherActor))

(event EventTick
  (params (DeltaSeconds :type Float%20%28single-precision%29))
  (bind _returnvalue (Subsystems|GetGameManagerWSS))
  (|CallParentFunction DeltaSeconds)
  (if (Variables|Default|GetCurrentlyActive)
    (Utilities|FlowControl|Sequence
      (:then_0
        (if (Variables|Default|GetlookingForPress)
          (bind _asbp_exit_shop_button (Utilities|Casting|CastToBP_ExitShopButton (Variables|/Script/Engine.ChildActorComponent|GetChildActor (Variables|Default|GetBP_ExitShopButton))))
          (bind _waspressed (Default|WasButtonPressed _asbp_exit_shop_button))
          (if _waspressed
            (Variables|Default|SetopeningExitDoors true)
            (Variables|Default|SetlookingForPress false)
            (Audio|SpawnSoundatLocation "/Game/Audio/MetaSounds/Door_Source.Door_Source" (+ (Transformation|GetWorldLocation (Variables|Default|GetDoorway_WALLS1)) "0.000000,0.000000,200.000000") "0, 0, 0" 1.0 1.0 0.0 0 0))))
      (:then_1
        (if (Variables|Default|GetopeningExitDoors)
          (bind _doorsopen (CallFunction|OpenShopDoors (Variables|Default|GetLeftShopExitDoor) (Variables|Default|GetRightShopExitDoor)))
          (if _doorsopen
            (Variables|Default|SetopeningExitDoors false)
            (Class|GameManagerWSS|ExitStation _returnvalue)
            (Variables|Default|SetCurrentlyActive false))))
      (:then_2
        (if (Variables|/Script/Prototype0Unreal.GameManagerWSS|GetwaitingForShopEnterDoors _returnvalue)
          (if (not (Variables|Default|GetopeningEnterDoors))
            (Variables|Default|SetopeningEnterDoors true)
            (Audio|SpawnSoundatLocation "/Game/Audio/MetaSounds/Door_Source.Door_Source" (+ (Transformation|GetWorldLocation (Variables|Default|GetDoorway_WALLS)) "0.000000,0.000000,200.000000") "0, 0, 0" 1.0 1.0 0.0 0 0))))
      (:then_3
        (if (Variables|Default|GetopeningEnterDoors)
          (bind _doorsopen_2 (CallFunction|OpenShopDoors (Variables|Default|GetshopEnterDoorLeft) (Variables|Default|GetshopEnterDoorRight)))
          (if _doorsopen_2
            (Variables|Default|SetopeningEnterDoors false)
            (Class|GameManagerWSS|EnterStation _returnvalue)
            (Variables|/Script/Prototype0Unreal.GameManagerWSS|SetwaitingForShopEnterDoors _returnvalue false)
            (Development|PrintString "Horde Defeated!")))))))

(fn ConstructionScript
  (|CallParentFunction))

(fn GetLength
  (bind _length_out (|CallParentFunction))
  (return (+ (* (.y (Transformation|GetWorldScale (Variables|Default|Getstation%20floor))) 1e+02) _length_out)))

(fn OpenShopDoors
  (params (LeftDoor :type Static%20Mesh%20Component%20Object%20Reference) (RightDoor :type Static%20Mesh%20Component%20Object%20Reference))
  (Transformation|SetWorldLocation RightDoor (+ (Transformation|GetWorldLocation RightDoor) (* (Math|Vector|MakeVector -1.0 0.0 0.0) (Variables|Default|GetDoorSpeed))) false false)
  (Transformation|SetWorldLocation LeftDoor (+ (Transformation|GetWorldLocation LeftDoor) (* (Math|Vector|MakeVector 1.0 0.0 0.0) (Variables|Default|GetDoorSpeed))) false false)
  (if (>= (.x (Transformation|GetWorldLocation LeftDoor)) (Variables|Default|GetExitDoorOpenedXVal))
    (return true)))