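; Enemy spawner Blueprint that, as wired, only drives encounter UI: a kill counter and a "survive the horde" warning.
; BeginPlay adds both component widgets to the viewport hidden and sets an enemies-per-chunk value.
; Events show or hide the counter with the needed kill count, or activate the warning with a 2D sound.
; Spawning is disconnected: NotifySpawnEnemy and SpawnEnemy are empty, leaving the AI_Enemy spawn, stat setup and targeting logic unreachable.
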(event EventBeginPlay
  (bind _killcounter (Variables|Default|GetKillCounter))
  (bind _hordewarning (Variables|Default|GetHordeWarning))
  (bind _returnvalue (UserInterface|GetWidget _killcounter))
  (bind _returnvalue_2 (UserInterface|GetWidget _hordewarning))
  (Variables|Default|SetEnemiesPerChunk 4)
  (UserInterface|Viewport|AddtoViewport _returnvalue 0)
  (UserInterface|Viewport|AddtoViewport _returnvalue_2 2)
  (Widget|SetVisibility _returnvalue "Hidden")
  (Widget|SetVisibility _returnvalue_2 "Hidden"))

(event Collision|EventActorBeginOverlap
  (params (OtherActor :type Actor%20Object%20Reference)))

(event EventTick
  (params (DeltaSeconds :type Float%20%28single-precision%29)))

(event EventNotifySpawnEnemy
  (params (spawnLocation :type Vector :default "0, 0, 0") (rotation :type Rotator :default "0, 0, 0") (SetTarget :type Boolean) (target :type Vector :default "0, 0, 0")))

(event EventDisplayKillCounter
  (params (enemiesNeeded :type Integer))
  (bind _killcounter (Variables|Default|GetKillCounter))
  (bind _returnvalue (UserInterface|GetWidget _killcounter))
  (Widget|SetVisibility _returnvalue "Visible")
  (bind _asencounter_kill_counter (Utilities|Casting|CastToEncounterKillCounter _returnvalue))
  (Default|SetText _asencounter_kill_counter (Utilities|Text|ToText(Integer) enemiesNeeded)))

(event EventHideKillCounter
  (Widget|SetVisibility (UserInterface|GetWidget (Variables|Default|GetKillCounter)) "Hidden"))

(event EventDisplayHordeWarning
  (bind _hordewarning (Variables|Default|GetHordeWarning))
  (bind _returnvalue (UserInterface|GetWidget _hordewarning))
  (Widget|SetVisibility _returnvalue "Visible")
  (bind _assurvive_the_horde (Utilities|Casting|CastToSurviveTheHorde _returnvalue))
  (Default|Activate _assurvive_the_horde)
  (Audio|PlaySound2D "/Game/Audio/AudioFiles/Enemies/HordeIncoming.HordeIncoming" 0.4 1.0 0.0 0 0))

(fn ConstructionScript)

(fn SpawnEnemy
  (params (spawnLocation :type Vector) (rotation :type Rotator) (setTargetImediatly :type Boolean) (target :type Vector)))