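; BP_RangedEnemy is a ranged enemy actor that uses obstacle health and damage events to drive a widget health bar.
; On BeginPlay it sets the bar's world yaw to a fixed value once to face the camera, then fills it.
; Damage notifications refresh the bar from current over max obstacle health, and ObstacleDestroyed destroys the actor.
; No attack logic lives in this graph.
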(event EventBeginPlay
  (CallFunction|HealthBarFaceCamera)
  (CallFunction|UpdateHealthBar))

(event Collision|EventActorBeginOverlap
  (params (OtherActor :type Actor%20Object%20Reference)))

(event EventTick
  (params (DeltaSeconds :type Float%20%28single-precision%29)))

(event EventNotifyDamageObstacle
  (CallFunction|UpdateHealthBar))

(event EventObstacleDestroyed
  (Actor|DestroyActor))

(fn ConstructionScript)

(fn HealthBarFaceCamera
  (bind _hb (Variables|Default|Gethb))
  (bind _returnvalue (Transformation|GetWorldRotation _hb))
  (Transformation|SetWorldRotation _hb (Math|Rotator|MakeRotator (.roll _returnvalue) (.pitch _returnvalue) -1.8e+02) false false))

(fn UpdateHealthBar
  (bind _aswb_health_bar (Utilities|Casting|CastToWB_HealthBar (UserInterface|GetWidget (Variables|Default|Gethb))))
  (Progress|SetPercent (Variables|/Game/Widgets/WB_HealthBar.WB_HealthBar_C|GetHealthBar _aswb_health_bar) (/ (Variables|Default|GetcurrentHealth) (Variables|Default|GetMaxObstacleHealth))))