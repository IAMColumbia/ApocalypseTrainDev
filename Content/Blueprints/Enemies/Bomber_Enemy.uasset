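; Bomber enemy Blueprint that carries two TNT bundle props in its hands.
; On BeginPlay it runs the parent logic, then attaches the bundles to the left and right item sockets on its mesh.
; Tick only forwards to the parent, and no explosion or attack logic appears here.
; A mesh-scaling snippet that stores InitialScale is left unconnected and never runs.
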(event EventBeginPlay
  (|CallParentFunction)
  (Transformation|AttachComponentToComponent (Variables|Default|GetTntBundleGameReady2) (Variables|Character|GetMesh) "RightItemSocket" "KeepWorld" "KeepWorld" "KeepRelative" false)
  (Transformation|AttachComponentToComponent (Variables|Default|GetTntBundleGameReady1) (Variables|Character|GetMesh) "LeftItemSocket" "KeepWorld" "KeepWorld" "KeepRelative" false))

(event Collision|EventActorBeginOverlap
  (params (OtherActor :type Actor%20Object%20Reference)))

(event EventTick
  (params (DeltaSeconds :type Float%20%28single-precision%29))
  (|CallParentFunction DeltaSeconds))

(fn ConstructionScript)