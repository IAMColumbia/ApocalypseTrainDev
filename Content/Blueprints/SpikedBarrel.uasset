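; Spiked barrel hazard that punishes enemies knocked into it.
; When an EnemyCharacter overlaps the Box while flagged WasKnocked, it takes damage equal to half its max health.
; Each hit switches both meshes to a bloody spike material and replays a timeline that scales Cube relative to its BeginPlay scale.
; An overlap-polling damage loop is left disconnected and never runs.
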(event OnComponentBeginOverlap(Box)
  (params (OverlappedComponent :type Primitive%20Component%20Object%20Reference) (OtherActor :type Actor%20Object%20Reference) (OtherComp :type Primitive%20Component%20Object%20Reference) (OtherBodyIndex :type Integer) (bFromSweep :type Boolean) (SweepResult :type Hit%20Result%20Structure%20%28by%20ref%29))
  (bind _asenemy_character (Utilities|Casting|CastToEnemyCharacter OtherActor))
  (Utilities|IsValid _asenemy_character
    (:Is%20Valid
      (if (Variables|/Script/Prototype0Unreal.EnemyCharacter|GetWasKnocked _asenemy_character)
        (Class|EnemyCharacter|TakeDamage _asenemy_character 0.0 (/ (Variables|/Script/Prototype0Unreal.EnemyCharacter|GetMaxHealth _asenemy_character) 2.0) "0, 0, 0" 0.0)
        (Rendering|Material|SetMaterial (Variables|Default|GetCube1) 0 "/Game/Models/SpikeTrapBLOODY_Mat.SpikeTrapBLOODY_Mat")
        (Rendering|Material|SetMaterial (Variables|Default|GetCube) 0 "/Game/Models/SpikeTrapBLOODY_Mat.SpikeTrapBLOODY_Mat")
        (bind _newtrack_1 (Timeline|Timeline_0 PlayFromStart)
          (:Update
            (Transformation|SetWorldScale3D (Variables|Default|GetCube) (* (Variables|Default|GetInitialScale) _newtrack_1))))))))

(event EventBeginPlay
  (Variables|Default|SetInitialScale (Transformation|GetWorldScale (Variables|Default|GetCube))))

(event Collision|EventActorBeginOverlap
  (params (OtherActor :type Actor%20Object%20Reference)))

(event EventTick
  (params (DeltaSeconds :type Float%20%28single-precision%29)))

(fn ConstructionScript)