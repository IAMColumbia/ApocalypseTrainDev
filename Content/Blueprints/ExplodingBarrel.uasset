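; Destructible exploding barrel obstacle with a world-space health bar that updates when damaged and has its yaw fixed at BeginPlay.
; On destruction it leaves a fading scorch decal, plays a pitch-varied sound and Niagara explosion, then destroys itself.
; The blast damages overlapping players at quarter strength, and BP_Shatter obstacles and enemies at full strength.
; Line-trace cover checks and enemy knockback exist but are disconnected, so cover is ignored.
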(event EventBeginPlay
  (CallFunction|HealthBarFaceCamera)
  (CallFunction|UpdateHealthBar))

(event Collision|EventActorBeginOverlap
  (params (OtherActor :type Actor%20Object%20Reference)))

(event EventTick
  (params (DeltaSeconds :type Float%20%28single-precision%29)))

(event EventNotifyDamageObstacle
  (params (damage :type Float%20%28single-precision%29))
  (CallFunction|UpdateHealthBar))

(event EventObstacleDestroyed
  (CallFunction|SpawnDecal)
  (CallFunction|Explosion))

(fn ConstructionScript)

(fn HealthBarFaceCamera
  (bind _hb (Variables|Default|Gethb))
  (bind _returnvalue (Transformation|GetWorldRotation _hb))
  (Transformation|SetWorldRotation _hb (Math|Rotator|MakeRotator (.roll _returnvalue) (.pitch _returnvalue) -1.8e+02) false false))

(fn UpdateHealthBar
  (bind _aswb_health_bar (Utilities|Casting|CastToWB_HealthBar (UserInterface|GetWidget (Variables|Default|Gethb))))
  (Progress|SetPercent (Variables|/Game/Widgets/WB_HealthBar.WB_HealthBar_C|GetHealthBar _aswb_health_bar) (/ (Variables|Default|GetcurrentHealth) (Variables|Default|GetMaxObstacleHealth))))

(fn Explosion
  (bind _explosionradius (Variables|Default|GetExplosionRadius))
  (Audio|SpawnSoundatLocation "/Game/Audio/MetaSounds/Grenade_Source.Grenade_Source" (Transformation|GetWorldLocation (Variables|Default|GetBarrellMesh)) "0, 0, 0" 1.0 (+ (Math|Random|RandomFloatinRange -0.1 0.1) 1.0) 0.0 "/Game/Audio/BasicAttenuation.BasicAttenuation" 0)
  (Utilities|FlowControl|Sequence
    (:then_0
      (Niagara|SpawnSystematLocation "/Game/VFX/Smoke_Explosion/NS_Explosion.NS_Explosion" (+ (Transformation|GetWorldLocation (Variables|Default|GetBarrellMesh)) "0.000000,0.000000,80.000000")))
    (:then_1
      (for _array_element (Collision|GetOverlappingActors _explosionradius "/Script/Prototype0Unreal.MyCharacter" :!class /Script/Engine.PrimitiveComponent)
        (bind _asmy_character (Utilities|Casting|CastToMyCharacter _array_element))
        (Class|MyCharacter|TakeDamage _asmy_character (/ (Variables|Default|GetDamage) 4.0) 1.0)))
    (:then_2
      (for _array_element_2 (Collision|GetOverlappingActors _explosionradius "/Game/Blueprints/BP_Shatter.BP_Shatter_C" :!class /Script/Engine.PrimitiveComponent)
        (bind _asbp_shatter (Utilities|Casting|CastToBP_Shatter _array_element_2))
        (Class|Obstacle|DamageObstacle _asbp_shatter (* (Variables|Default|GetDamage) 1.0))))
    (:then_3
      (for _array_element_3 (Collision|GetOverlappingActors _explosionradius "/Script/Prototype0Unreal.EnemyCharacter" :!class /Script/Engine.PrimitiveComponent)
        (bind _asenemy_character (Utilities|Casting|CastToEnemyCharacter _array_element_3))
        (Class|EnemyCharacter|TakeDamage _asenemy_character 0.0 (Variables|Default|GetDamage) "0, 0, 0" 0.0 true)))
    (:then_4
      (Actor|DestroyActor))))

(fn HasCover
  (params (Actor :type Actor%20Object%20Reference))
  (bind _returnvalue (Transformation|GetActorLocation))
  (bind _barrellmesh (Variables|Default|GetBarrellMesh))
  (bind _returnvalue_2 (Transformation|GetWorldLocation _barrellmesh))
  (Utilities|IsValid Actor
    (:Is%20Valid
      (Utilities|Array|Add (Variables|Default|GetActors%20to%20Ignore) Actor)
      (bind _returnvalue_3 (Collision|LineTraceByChannel _returnvalue _returnvalue_2 "TraceTypeQuery1" false (Variables|Default|GetActors%20to%20Ignore) "None"))
      (return _returnvalue_3 (Math|Vector|Normalize (- _returnvalue_2 _returnvalue))))))

(fn SpawnDecal
  (bind _returnvalue (Rendering|Decal|SpawnDecalatLocation "/Game/Decals/ExplosionHole_Mat.ExplosionHole_Mat" (Math|Conversions|ToVector(Float) (Math|Float|MakeLiteralFloat 1.2e+02)) (Transformation|GetWorldLocation (Variables|Default|GetBarrellMesh)) (Math|Rotator|MakeRotator 0.0 -9e+01 (Math|Random|RandomFloatinRange -1.8e+02 1.8e+02)) 0.0))
  (Rendering|Components|Decal|SetFadeOut _returnvalue 2.0 3.0 true))