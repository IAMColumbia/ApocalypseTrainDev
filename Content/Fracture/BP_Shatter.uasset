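; Destructible barricade obstacle built on a Geometry Collection, with a widget health bar.
; On each damage notification it updates the bar, flashes white through a dynamic material and plays a timeline scale pulse.
; At zero health it disables its box collision, hides the bar and spawns a Damage actor at the collection.
; A separate ObstacleDestroyed event dissolves the material on a timeline, then destroys the actor.
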(event OnEndCursorOver(Barricade3_GeometryCollection)
  (params (TouchedComponent :type Primitive%20Component%20Object%20Reference)))

(event OnChaosBreakEvent(Barricade3_GeometryCollection)
  (params (BreakEvent :type Chaos%20Break%20Event%20Structure%20%28by%20ref%29)))

(event OnComponentBeginOverlap(Box)
  (params (OverlappedComponent :type Primitive%20Component%20Object%20Reference) (OtherActor :type Actor%20Object%20Reference) (OtherComp :type Primitive%20Component%20Object%20Reference) (OtherBodyIndex :type Integer) (bFromSweep :type Boolean) (SweepResult :type Hit%20Result%20Structure%20%28by%20ref%29))
  (if (Actor|ActorHasTag OtherActor "Player")
    _))

(event EventBeginPlay
  (CallFunction|UpdateHealthBar)
  (bind _returnvalue (Rendering|Material|CreateDynamicMaterialInstance (Variables|Default|GetBarricade3_GeometryCollection) 0 "/Game/Mesh/StreetProps/Barricade2.Barricade2" "FlashMat" :!class /Script/Engine.PrimitiveComponent))
  (bind _output_get (Variables|Components|SetFlashMat _returnvalue))
  (Rendering|Material|SetVectorParameterValue _output_get "FlashVector" (Math|Conversions|ToLinearColor(Vector) (Math|Vector|MakeVector 0.0 0.0 0.0)) :!class /Script/Engine.MaterialInstanceDynamic)
  (Variables|Components|SetScale (Transformation|GetWorldScale (Variables|Default|GetBarricade3_GeometryCollection))))

(event EventObstacleDestroyed
  (bind _newtrack_0 (Timeline|Timeline_0 PlayFromStart)
    (:Update
      (Rendering|Material|SetScalarParameterValue (Variables|Components|GetFlashMat) "Dissolve" _newtrack_0 :!class /Script/Engine.MaterialInstanceDynamic))
    (:Finished
      (Actor|DestroyActor))))

(event EventTick
  (params (DeltaSeconds :type Float%20%28single-precision%29)))

(event EventNotifyDamageObstacle
  (bind _box (Variables|Default|GetBox))
  (bind _flashmat (Variables|Components|GetFlashMat))
  (CallFunction|UpdateHealthBar)
  (Utilities|FlowControl|Sequence
    (:then_0
      (Rendering|Material|SetVectorParameterValue _flashmat "FlashVector" (Math|Conversions|ToLinearColor(Vector) (Math|Vector|MakeVector 1.0 1.0 1.0)) :!class /Script/Engine.MaterialInstanceDynamic)
      (Utilities|FlowControl|Delay 0.1)
      (Rendering|Material|SetVectorParameterValue _flashmat "FlashVector" (Math|Conversions|ToLinearColor(Vector) (Math|Vector|MakeVector 0.0 0.0 0.0)) :!class /Script/Engine.MaterialInstanceDynamic))
    (:then_1
      (bind _newtrack_1 (Timeline|Timeline PlayFromStart)
        (:Update
          (Transformation|SetWorldScale3D (Variables|Default|GetBarricade3_GeometryCollection) (* (Variables|Components|GetScale) _newtrack_1)))))
    (:then_2
      (if (<= (Variables|Default|GetcurrentHealth) 0.0)
        (Collision|SetCollisionEnabled _box "NoCollision")
        (Components|Activation|SetActive _box false false)
        (Game|SpawnActorfromClass "/Game/Fracture/Damage.Damage_C" (Math|Transform|MakeTransform (Transformation|GetWorldLocation (Variables|Default|GetBarricade3_GeometryCollection)) "0, 0, 0" "1.000000,1.000000,1.000000") "Undefined" "MultiplyWithRoot" 0 0)
        (Rendering|SetVisibility (Variables|Default|Gethb) false false)))))

(event Collision|EventActorBeginOverlap
  (params (OtherActor :type Actor%20Object%20Reference)))

(fn ConstructionScript)

(fn UpdateHealthBar
  (bind _aswb_health_bar (Utilities|Casting|CastToWB_HealthBar (UserInterface|GetWidget (Variables|Default|Gethb))))
  (Progress|SetPercent (Variables|/Game/Widgets/WB_HealthBar.WB_HealthBar_C|GetHealthBar _aswb_health_bar) (/ (Variables|Default|GetcurrentHealth) (Variables|Default|GetMaxObstacleHealth))))